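; RoomDescription is a demo room display stand built from a base mesh and a flat wall mesh, tinted by StandColor.
; The construction script creates dynamic material instances on both meshes and sets their Color parameter.
; On BeginPlay, outside dedicated servers, it checks the first player controller's BP_InventoryComponent and makes both meshes block the Camera channel when the view is not top-down.
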(event `self.ReceiveBeginPlay`
  (bind _returnvalue (`self.GetComponentByClass` (`GameplayStatics.GetPlayerController` 0) "/Game/RPG/Blueprints/InventorySystem/Components/BP_InventoryComponent.BP_InventoryComponent_C"))
  (if (not (`KismetSystemLibrary.IsDedicatedServer`))
    (`/Engine/EditorBlueprintResources/StandardMacros.IsValid` _returnvalue
      (:`Is Valid`
        (if (not (`/Game/RPG/Blueprints/InventorySystem/Components/BP_InventoryComponent.IsTopDown` _returnvalue))
          (`PrimitiveComponent.SetCollisionResponseToChannel` (`self.SM_Base`) "ECC_Camera" "ECR_Block")
          (`PrimitiveComponent.SetCollisionResponseToChannel` (`self.SM_Base_FlatWall`) "ECC_Camera" "ECR_Block"))))))

(fn `UserConstructionScript`
  (bind _returnvalue (`PrimitiveComponent.CreateDynamicMaterialInstance` (`self.SM_Base`) 3 null "None"))
  (`MaterialInstanceDynamic.SetVectorParameterValue` _returnvalue "Color" (`self.StandColor`))
  (bind _returnvalue_2 (`PrimitiveComponent.CreateDynamicMaterialInstance` (`self.SM_Base_FlatWall`) 0 null "None"))
  (`MaterialInstanceDynamic.SetVectorParameterValue` _returnvalue_2 "Color" (`self.StandColor`)))