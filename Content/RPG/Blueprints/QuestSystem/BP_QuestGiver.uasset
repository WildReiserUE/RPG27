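; BP_QuestGiver is an interactable quest-giving actor that players cannot damage.
; When its nameplate becomes visible, it toggles a quest icon on its AI healthbar widget, which also shows the interact key.
; Availability checks player level and quest status, recursively advancing completed quests along their chain.
; Interacting with an available quest checks talk-to objectives and opens a quest widget, refreshing the icon on close.
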(event `self.ReceiveBeginPlay`
  ;[1 1 1] Show quest icon if our player meets the requirements
  (`parent.ReceiveBeginPlay`)
  (`/Engine/EditorBlueprintResources/StandardMacros.IsValid` (`WidgetComponent.GetWidget` (`self.Widget`))
    (:`Is Valid`
      (add `/Game/RPG/Blueprints/InventorySystem/JigSaw/PickupSystem/BP_NameVisibility.OnVisibilityChanged` (`self.BP_NameVisibility`) (delegate `OnVisibilityChanged_Event_0`)))))

(event `OnVisibilityChanged_Event_0`
  (params (`Visible?` :type Boolean))
  ;[1 1 1] Show quest icon if our player meets the requirements
  (if `Visible?`
    (bind _result (`self.CheckIfQuestIsAvailable`))
    (bind _asbp_aihealthbar (cast `/Game/RPG/Blueprints/AI/Widgets/BP_AIHealthbar` (`WidgetComponent.GetWidget` (`self.Widget`))))
    (`/Game/RPG/Blueprints/AI/Widgets/BP_AIHealthbar.SetQuestVisibility` _asbp_aihealthbar _result)))

(event `/Game/RPG/Blueprints/OtherBlueprints/IT_InteractInterface.ExecuteInteract`
  (params (CharacterRef :type "Actor Object Reference") (Comp :type "/Game/RPG/Blueprints/InventorySystem/Components/BP_InventoryComponent Object Reference"))
  ;[1 1 1] Interacting with the quest actor
  (`parent.ExecuteInteract` CharacterRef Comp)
  (bind _result (`self.CheckIfQuestIsAvailable`))
  (if _result
    (bind _comp (message `/Game/RPG/Blueprints/Character/Interfaces/BP_QuestInterface.GetQuestComponent` (`ActorComponent.GetOwner` Comp)))
    (`/Game/RPG/Blueprints/QuestSystem/BP_PlayerQuestComponent.CheckIfTalkToObjective` _comp self)
    (bind _returnvalue (`|CreateWidget` "/Game/RPG/Blueprints/QuestSystem/Widgets/BP_QuestWidget.BP_QuestWidget_C" null (`/Game/RPG/Blueprints/QuestSystem/BP_QuestInfoComponent.GetQuestInfo` (`self.BP_QuestInfoComponent`)) _comp self))
    (`/Game/RPG/Blueprints/InventorySystem/Components/BP_InventoryComponent.AddContent` Comp _returnvalue)
    (`/Game/RPG/Blueprints/InventorySystem/Components/BP_InventoryComponent.ShowInventory` Comp)
    (add `/Game/RPG/Blueprints/QuestSystem/Widgets/BP_QuestWidget.Closed` _returnvalue (delegate `Closed_Event_0`))))

(event `Closed_Event_0`
  ;[1 1 1] Interacting with the quest actor
  (`/Engine/EditorBlueprintResources/StandardMacros.IsValid` (stale `/Game/RPG/Blueprints/OtherBlueprints/IT_InteractInterface.ExecuteInteract` Comp)
    (:`Is Valid`
      (`/Game/RPG/Blueprints/InventorySystem/Components/BP_InventoryComponent.RemoveContent` (stale `/Game/RPG/Blueprints/OtherBlueprints/IT_InteractInterface.ExecuteInteract` Comp))
      (`self.OnVisibilityChanged_Event_0` true))))

(fn `CanBeDamagedByPlayer?`
  (returns (Result :type Boolean))
  (return false))

(fn `CheckIfQuestIsAvailable`
  (returns (Result :type Boolean))
  (locals (`QuestAvailable?` :type Boolean :default false))
  (bind ((`QuestUniqueID_32_3B494E2D4A23FB4179D078807AC2F1ED` _questuniqueid) (`ChainsToQuest_47_0CAA47E74D67B89957C38F800DC8E8A9` _chainstoquest) (`LevelRequired_6_4072C83D415B10B5F16DD1A462692AF7` _levelrequired)) (break `/Game/RPG/Blueprints/QuestSystem/QuestCreator/Data/S_QuestInfo` (`/Game/RPG/Blueprints/QuestSystem/BP_QuestInfoComponent.GetQuestInfo` (`self.BP_QuestInfoComponent`))))
  (`|ExecutionSequence`
    (:`then_0`
      (bind _actorref (message `/Game/RPG/Blueprints/Character/Interfaces/BP_ARPGControllerInterface.GetControlledPawnRef` (`GameplayStatics.GetPlayerController` 0)))
      (`/Engine/EditorBlueprintResources/StandardMacros.IsValid` _actorref
        (:`Is Valid`
          (bind _level (message `/Game/RPG/Blueprints/Character/Interfaces/BP_CharacterInventoryInterface.JigGetPlayerLevel` _actorref))
          (if (>= _level _levelrequired)
            (bind _comp (message `/Game/RPG/Blueprints/Character/Interfaces/BP_QuestInterface.GetQuestComponent` (`GameplayStatics.GetPlayerController` 0)))
            (bind (_info _found_) (`/Game/RPG/Blueprints/QuestSystem/BP_PlayerQuestComponent.GetQuestByUID` _comp _questuniqueid))
            (set `local.QuestAvailable?` (or (not _found_) (`|EnumInequality` (`.CurrentStatus_6_C0B23D5F427B94BC5FAB6C982F190F9E` (break `/Game/RPG/Blueprints/QuestSystem/QuestCreator/Data/S_PlayerQuestStatus` _info)) "NewEnumerator1")))
            (`|ExecutionSequence`
              (:`then_0`
                (if (and (`|EnumEquality` (`.CurrentStatus_6_C0B23D5F427B94BC5FAB6C982F190F9E` (break `/Game/RPG/Blueprints/QuestSystem/QuestCreator/Data/S_PlayerQuestStatus` _info)) "NewEnumerator1") _found_ (!= _chainstoquest "None"))
                  (bind _output_get (`/Game/RPG/Blueprints/QuestSystem/BP_QuestInfoComponent.SetChainedQuest` (`self.BP_QuestInfoComponent`) _chainstoquest)) ; Set the new unique ID
                  (if _output_get
                    (bind _result (`self.CheckIfQuestIsAvailable`))
                    (return _result))))
              (:`then_1`
                (return (`local.QuestAvailable?`))))))))
    (:`then_1`
      (return false))))

(fn `OnQuestCompleted`
  (params (Player :type "Actor Object Reference") (QuestUID :type Name)))

(fn `SetOutlineEnabled`
  (params (Enabled :type Boolean) (InteractKey :type "Key Structure") (CalledFrom :type "Actor Object Reference"))
  (returns (`Enabled?` :type Boolean))
  (locals (NoneKey :type "Key Structure"))
  (bind _returnvalue (== InteractKey (`local.NoneKey`)))
  (bind _enabled_ (`parent.SetOutlineEnabled` Enabled InteractKey null))
  (`|ExecutionSequence`
    (:`then_0`
      (if (not _returnvalue)
        (bind _asbp_aihealthbar (cast `/Game/RPG/Blueprints/AI/Widgets/BP_AIHealthbar` (`WidgetComponent.GetUserWidgetObject` (`self.Widget`))))
        (`/Game/RPG/Blueprints/AI/Widgets/BP_AIHealthbar.SetInteractKey` _asbp_aihealthbar (`KismetInputLibrary.Key_GetDisplayName` InteractKey) (or _returnvalue (not Enabled)))))
    (:`then_1`
      (return _enabled_))))

(fn `UserConstructionScript`
  (`parent.UserConstructionScript`))