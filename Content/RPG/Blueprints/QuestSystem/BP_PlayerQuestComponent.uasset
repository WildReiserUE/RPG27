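; Player quest component that tracks accepted quests through server accept and complete requests, with save and load support.
; Replicated quest status is paired by index with non-replicated quest data to track kill, item, interact, area and gold objectives.
; Tracking functions update counts and re-evaluate completion, which can revert, then refresh the inventory's quest UI.
; Completion consumes required items and gold, grants XP, currency, skill points and items, then syncs the client by RPC.
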(event `SERVER_RequestAcceptQuest`
  (params (QuestGiver :type "/Game/RPG/Blueprints/QuestSystem/BP_QuestGiver Object Reference") (CurrentProgressUID :type Integer) (QuestUID :type Name))
  ;[1 1 1] Quest accepted
  (`/Engine/EditorBlueprintResources/StandardMacros.IsValid` QuestGiver
    (:`Is Valid`
      (bind (_info _found_) (`self.GetQuestByUID` QuestUID))
      (if (not _found_)
        (bind _out_row (`/Game/RPG/Blueprints/QuestSystem/BP_QuestInfoComponent.GetQuestInfoByUID` (`/Game/RPG/Blueprints/QuestSystem/BP_QuestGiver.BP_QuestInfoComponent` QuestGiver) QuestUID))
        (`self.AddNewQuest` CurrentProgressUID _out_row)
        (`KismetArrayLibrary.Array_Add` (`self.QuestDataNonRep`) _out_row)
        (`self.QuestTrack_OnInventoryItemsUpdated` true)))))

(event `SERVER_RequestCompleteQuest`
  (params (QuestGiver :type "/Game/RPG/Blueprints/QuestSystem/BP_QuestGiver Object Reference") (CurrentProgressUID :type Integer) (ItemAddedUID :type Integer) (ToIndex :type Integer) (`ItemRotated?` :type Boolean) (QuestUID :type Name))
  ;[1 1 1] Quest completed
  (`/Engine/EditorBlueprintResources/StandardMacros.IsValid` QuestGiver
    (:`Is Valid`
      (bind (_info _found_) (`self.GetQuestByUID` QuestUID))
      (if (and _found_ (`|EnumEquality` (`.CurrentStatus_6_C0B23D5F427B94BC5FAB6C982F190F9E` (break `/Game/RPG/Blueprints/QuestSystem/QuestCreator/Data/S_PlayerQuestStatus` _info)) "NewEnumerator2"))
        (`self.SetQuestStatusByID` QuestUID "NewEnumerator1" CurrentProgressUID)
        (bind _actorref (message `/Game/RPG/Blueprints/Character/Interfaces/BP_ARPGControllerInterface.GetControlledPawnRef` (`self.GetOwner`)))
        (`/Game/RPG/Blueprints/QuestSystem/BP_QuestGiver.OnQuestCompleted` QuestGiver _actorref QuestUID)
        (bind _out_row (`/Game/RPG/Blueprints/QuestSystem/BP_QuestInfoComponent.GetQuestInfoByUID` (`/Game/RPG/Blueprints/QuestSystem/BP_QuestGiver.BP_QuestInfoComponent` QuestGiver) QuestUID))
        (`self.ClaimRewards` ItemAddedUID ToIndex `ItemRotated?` _out_row)
        (`|ExecutionSequence`
          (:`then_0`
            (bind ((`QuestUniqueID_32_3B494E2D4A23FB4179D078807AC2F1ED` _questuniqueid) (`ResetQuestOnComplete_44_B0DA2E224075CFF9430CB1BCBCE971DA` _resetquestoncomplete)) (break `/Game/RPG/Blueprints/QuestSystem/QuestCreator/Data/S_QuestInfo` _out_row))
            (if _resetquestoncomplete
              (`self.AbandonQuest` _questuniqueid)))
          (:`then_1`
            (`self.CheckForcedRepNotify`)))))))

(event `SERVER_OnQuestGiverInteract`
  (params (QuestG :type "/Game/RPG/Blueprints/QuestSystem/BP_QuestGiver Object Reference"))
  ;[1 1 1] Interacted with a quest giver, it could be part of another quest
  (`self.QuestTrack_OnInteractedWith` QuestG))

(event `CLIENT_OnQuestCompleted`
  (params (ItemAddedUID :type Integer) (ConsumedUIDs :type "Array of Integer") (CountsToUpdate :type "Array of Integer") (NewCurrency :type "/Game/RPG/Blueprints/InventorySystem/JigSaw/Data/Structs/CharacterCurrency Structure") (SkillPointsEarned :type Integer))
  (bind _returnvalue (`self.GetOwner`))
  ;[1 1 1] On quest completed
  (bind _comp (message `/Game/RPG/Blueprints/Character/Interfaces/BP_ARPGControllerInterface.GetSkillTreeComponent` _returnvalue))
  (`/Game/RPG/Blueprints/Skills/Blueprint/SkillComponent/ClassSkillTree/BP_ClassSkillTreeComp.CLIENT_OnSkillPointsEarned` _comp SkillPointsEarned)
  (bind _inv (message `/Game/RPG/Blueprints/Character/Interfaces/BP_ARPGControllerInterface.GetInventoryComponent` _returnvalue))
  (`/Game/RPG/Blueprints/InventorySystem/Components/BP_InventoryComponent.ClientFunc_OnQuestCompleted` _inv ItemAddedUID ConsumedUIDs CountsToUpdate NewCurrency))

(fn `AbandonQuest`
  (params (QuestID :type Name))
  (returns (Result :type Boolean))
  (for (_array_element _array_index) (`self.PlayerQuests`)
    (if (== (`.UniqueQuestID_3_12E1AFAE40DEF67DD7A4F8A2397E8304` (break `/Game/RPG/Blueprints/QuestSystem/QuestCreator/Data/S_PlayerQuestStatus` _array_element)) QuestID)
      (`KismetArrayLibrary.Array_Remove` (`self.PlayerQuests`) _array_index)
      (return true)))
  (return false))

(fn `AddNewQuest`
  (params (CurrentProgressUID :type Integer) (Info :type "/Game/RPG/Blueprints/QuestSystem/QuestCreator/Data/S_QuestInfo Structure (by ref)"))
  (locals (Objectives :type "Array of /Game/RPG/Blueprints/QuestSystem/QuestCreator/Data/S_RepQuestObjective Structure") (Inv :type "/Game/RPG/Blueprints/InventorySystem/Components/BP_InventoryComponent Object Reference"))
  (bind ((`QuestUniqueID_32_3B494E2D4A23FB4179D078807AC2F1ED` _questuniqueid) (`ChainsToQuest_47_0CAA47E74D67B89957C38F800DC8E8A9` _chainstoquest) (`Objectives_26_348B948B4771E0192E317E911A007B98` _objectives)) (break `/Game/RPG/Blueprints/QuestSystem/QuestCreator/Data/S_QuestInfo` Info))
  (set `local.Inv` (`self.GetInventoryComponent`))
  (`|ExecutionSequence`
    (:`then_0`
      (for _array_element _objectives
        (bind ((`ObjectiveName_16_CA6E70DC48C56B7799C14DA5F98A54CC` _objectivename) (`ActionName_22_FACA197844ED72BCE7D9539BC9F5ADCE` _actionname) (`Type_2_88BA4D0B462FB1C99959DC93CF051C40` _type) (`Count_5_D69E848B40B7E925F5C1FCA7F2CC1B9E` _count) (`GiveGoldValue_19_652F1C874FC719F8784B1A815CE066A5` _givegoldvalue)) (break `/Game/RPG/Blueprints/QuestSystem/QuestCreator/Data/S_QuestObjective` _array_element))
        (`KismetArrayLibrary.Array_Add` (`local.Objectives`) (make `/Game/RPG/Blueprints/QuestSystem/QuestCreator/Data/S_RepQuestObjective` _type 0.0 (`KismetMathLibrary.SelectFloat` (`/Game/RPG/Blueprints/InventorySystem/Components/BP_InventoryComponent.GetTotalGoldInFloat` (`local.Inv`) _givegoldvalue 0.0) (`KismetMathLibrary.Conv_IntToDouble` (`KismetMathLibrary.SelectInt` 1 _count (< _count 1))) (`|EnumEquality` _type "NewEnumerator4")) _objectivename))))
    (:`then_1`
      (`KismetArrayLibrary.Array_Add` (`self.PlayerQuests`) (make `/Game/RPG/Blueprints/QuestSystem/QuestCreator/Data/S_PlayerQuestStatus` _questuniqueid "NewEnumerator0" CurrentProgressUID (`local.Objectives`)))
      (`self.CheckForcedRepNotify`))))

(fn `CheckForcedRepNotify`
  (bind _inv (message `/Game/RPG/Blueprints/Character/Interfaces/BP_ARPGControllerInterface.GetInventoryComponent` (`self.GetOwner`)))
  (bind _maininventoryref (`/Game/RPG/Blueprints/InventorySystem/Components/BP_InventoryComponent.GetInventoryRef` _inv))
  (`/Engine/EditorBlueprintResources/StandardMacros.IsValid` _maininventoryref
    (:`Is Valid`
      (`/Game/RPG/Widgets/BP_MainInventory.RefreshQuests` _maininventoryref))))

(fn `CheckForCompletedQuests`
  (locals (Failed :type Boolean))
  (for _index (range (`KismetArrayLibrary.Array_Length` (`self.PlayerQuests`)))
    (bind ((`CurrentStatus_6_C0B23D5F427B94BC5FAB6C982F190F9E` _currentstatus) (`Objectives_13_7573456046651D48DA23EAA039CEFA45` _objectives)) (break `/Game/RPG/Blueprints/QuestSystem/QuestCreator/Data/S_PlayerQuestStatus` (`|GetArrayItem` (`self.PlayerQuests`) _index)))
    (if (`|EnumInequality` _currentstatus "NewEnumerator1")
      (set `local.Failed` false)
      (for _array_element _objectives
        (bind ((`CurrentCount_20_D69E848B40B7E925F5C1FCA7F2CC1B9E` _currentcount) (`ObjectiveCount_21_4E02AFDD4BC542F68100068E434E6F04` _objectivecount)) (break `/Game/RPG/Blueprints/QuestSystem/QuestCreator/Data/S_RepQuestObjective` _array_element))
        (if (< _currentcount _objectivecount)
          (set `local.Failed` true)
          (break)))
      (setmembers `/Game/RPG/Blueprints/QuestSystem/QuestCreator/Data/S_PlayerQuestStatus` :`StructRef` (`|GetArrayItem` (`self.PlayerQuests`) _index) :`CurrentStatus` (select `bool` (`local.Failed`) :`false` "NewEnumerator2" :`true` "NewEnumerator0" :!type "/Game/RPG/Blueprints/QuestSystem/QuestCreator/Data/E_QuestStatus Enum"))))
  (`self.CheckForcedRepNotify`))

(fn `CheckIfTalkToObjective`
  (params (QuestG :type "/Game/RPG/Blueprints/QuestSystem/BP_QuestGiver Object Reference"))
  (for _array_element (`self.PlayerQuests`)
    (bind ((`CurrentStatus_6_C0B23D5F427B94BC5FAB6C982F190F9E` _currentstatus) (`Objectives_13_7573456046651D48DA23EAA039CEFA45` _objectives)) (break `/Game/RPG/Blueprints/QuestSystem/QuestCreator/Data/S_PlayerQuestStatus` _array_element))
    (if (`|EnumEquality` _currentstatus "NewEnumerator0")
      (for _array_element_2 _objectives
        (if (`|EnumEquality` (`.Type_2_88BA4D0B462FB1C99959DC93CF051C40` (break `/Game/RPG/Blueprints/QuestSystem/QuestCreator/Data/S_RepQuestObjective` _array_element_2)) "NewEnumerator2")
          (`self.SERVER_OnQuestGiverInteract` (`local.QuestG`))
          (return))))))

(fn `ClaimRewards`
  (params (ItemUID :type Integer) (Index :type Integer) (Rotated :type Boolean) (QuestInfo :type "/Game/RPG/Blueprints/QuestSystem/QuestCreator/Data/S_QuestInfo Structure"))
  (locals (ItemsToConsume :type "Array of Name") (ItemCounts :type "Array of Integer") (UIDsToUpdate :type "Array of Integer") (CountsToUpdate :type "Array of Integer") (NewCurrency :type "/Game/RPG/Blueprints/InventorySystem/JigSaw/Data/Structs/CharacterCurrency Structure") (InvCom :type "/Game/RPG/Blueprints/InventorySystem/Components/BP_InventoryComponent Object Reference"))
  (bind ((`QuestDescription_41_BB7FA9CC4A6E3488D32BC18C2BA50330` _questdescription) (`ChainsToQuest_47_0CAA47E74D67B89957C38F800DC8E8A9` _chainstoquest) (`ExpEarned_9_A04646E24D05D9CB714DF78880F85584` _expearned) (`CurrencyEarned_15_5617E0A94BEA34E7A4E910975D4582FF` _currencyearned) (`SkillPointsEarned_35_B7D3C6454E867C62514D0EB6487F3AF2` _skillpointsearned) (`ItemIDEarned_19_22B1AED5465A77904D3E12A0C2BB3954` _itemidearned) (`ItemEarnedCount_38_6DEA279A4E68B5D7FD9E0E9A20821A9E` _itemearnedcount) (`ItemDataTable_22_6990F0C5480204C30DCF9086BF2D3F3E` _itemdatatable)) (break `/Game/RPG/Blueprints/QuestSystem/QuestCreator/Data/S_QuestInfo` QuestInfo))
  (bind _returnvalue (`self.GetOwner`))
  (bind _actorref (message `/Game/RPG/Blueprints/Character/Interfaces/BP_ARPGControllerInterface.GetControlledPawnRef` _returnvalue))
  (message `/Game/RPG/Blueprints/Skills/Blueprint/SkillComponent/IT_SkillEffects.Skill_OnTargetExpEarned` _actorref null _expearned false)
  (bind _inv (message `/Game/RPG/Blueprints/Character/Interfaces/BP_ARPGControllerInterface.GetInventoryComponent` _returnvalue))
  (set `local.InvCom` _inv)
  (`|ExecutionSequence`
    (:`then_0`
      (for _array_element (`.Objectives_26_348B948B4771E0192E317E911A007B98` (break `/Game/RPG/Blueprints/QuestSystem/QuestCreator/Data/S_QuestInfo` QuestInfo))
        (bind ((`ActionName_22_FACA197844ED72BCE7D9539BC9F5ADCE` _actionname) (`Type_2_88BA4D0B462FB1C99959DC93CF051C40` _type) (`Count_5_D69E848B40B7E925F5C1FCA7F2CC1B9E` _count) (`OrTagID_13_73AF88824DDC4605B8744094D5240D65` _ortagid) (`GiveGoldValue_19_652F1C874FC719F8784B1A815CE066A5` _givegoldvalue)) (break `/Game/RPG/Blueprints/QuestSystem/QuestCreator/Data/S_QuestObjective` _array_element))
        (if (`|EnumEquality` _type "NewEnumerator1")
          (`KismetArrayLibrary.Array_Add` (`local.ItemsToConsume`) _ortagid)
          (`KismetArrayLibrary.Array_Add` (`local.ItemCounts`) _count)
          (elif (`|EnumEquality` _type "NewEnumerator4")
            (bind _output_get (`/Game/RPG/Blueprints/InventorySystem/Components/BP_InventoryComponent.RemoveCurrency` (`local.InvCom`) _givegoldvalue))
            (set `local.NewCurrency` _output_get))))
      (if (`KismetArrayLibrary.Array_IsValidIndex` (`local.ItemsToConsume`))
        (bind _updatedinvvalues (`/Game/RPG/Blueprints/InventorySystem/Components/BP_InventoryComponent.ServerFunc_ConsumeItems` (`local.InvCom`) (`local.ItemsToConsume`) (`local.ItemCounts`)))
        (bind _values (`BlueprintMapLibrary.Map_Values` _updatedinvvalues))
        (set `local.CountsToUpdate` _values)
        (bind _keys (`BlueprintMapLibrary.Map_Keys` _updatedinvvalues))
        (set `local.UIDsToUpdate` _keys)))
    (:`then_1`
      (bind _output_get_2 (`/Game/RPG/Blueprints/InventorySystem/Components/BP_InventoryComponent.AddCurrency` (`local.InvCom`) _currencyearned))
      (set `local.NewCurrency` _output_get_2)
      (bind _comp (message `/Game/RPG/Blueprints/Character/Interfaces/BP_ARPGControllerInterface.GetSkillTreeComponent` _returnvalue))
      (`/Game/RPG/Blueprints/Skills/Blueprint/SkillComponent/ClassSkillTree/BP_ClassSkillTreeComp.OnSkillPointGained` _comp _skillpointsearned)
      (`|ExecutionSequence`
        (:`then_0`
          (if (!= _itemidearned "None")
            (`/Game/RPG/Blueprints/InventorySystem/Components/BP_InventoryComponent.ServerFunc_AddItemToInventory` (`local.InvCom`) _itemidearned _itemearnedcount _itemdatatable (`local.ItemUID`) (`local.Index`) (`local.Rotated`))))
        (:`then_1`
          (`self.CLIENT_OnQuestCompleted` (`local.ItemUID`) (`local.UIDsToUpdate`) (`local.CountsToUpdate`) (`local.NewCurrency`) (`/Game/RPG/Blueprints/Skills/Blueprint/SkillComponent/ClassSkillTree/BP_ClassSkillTreeComp.CurrentSkillPoints` _comp))
          (return))))))

(fn `GetCurrentQuestUIDs`
  (returns (QuestUIDS :type "Array of Name"))
  (locals (UIDs :type "Array of Name"))
  (`KismetArrayLibrary.Array_Clear` (`local.UIDs`))
  (for _array_element (`self.PlayerQuests`)
    (`KismetArrayLibrary.Array_Add` (`local.UIDs`) (`.UniqueQuestID_3_12E1AFAE40DEF67DD7A4F8A2397E8304` (break `/Game/RPG/Blueprints/QuestSystem/QuestCreator/Data/S_PlayerQuestStatus` _array_element))))
  (return (`local.UIDs`)))

(fn `GetInventoryComponent`
  (returns (Inv :type "/Game/RPG/Blueprints/InventorySystem/Components/BP_InventoryComponent Object Reference"))
  (bind _inv (message `/Game/RPG/Blueprints/Character/Interfaces/BP_ARPGControllerInterface.GetInventoryComponent` (`self.GetOwner`)))
  (return _inv))

(fn `GetQuestByUID`
  (params (QuestUID :type Name))
  (returns (Info :type "/Game/RPG/Blueprints/QuestSystem/QuestCreator/Data/S_PlayerQuestStatus Structure") (`Found?` :type Boolean))
  (for _array_element (`self.PlayerQuests`)
    (if (== (`.UniqueQuestID_3_12E1AFAE40DEF67DD7A4F8A2397E8304` (break `/Game/RPG/Blueprints/QuestSystem/QuestCreator/Data/S_PlayerQuestStatus` _array_element)) (`local.QuestUID`))
      (return _array_element true)))
  (return (struct) false))

(fn `LoadSaves`
  (params (SaveData :type "/Game/RPG/Blueprints/InventorySystem/SaveSystem/SaveData Structure (by ref)"))
  (returns (Result :type Boolean))
  (bind ((`Quests_69_1F472F374F16C44B27A2CAB448778FD3` _quests) (`QuestsInfo_74_6A8D69D248F347480051A592FB5C6126` _questsinfo)) (break `/Game/RPG/Blueprints/InventorySystem/SaveSystem/SaveData` SaveData))
  (set `self.PlayerQuests` _quests)
  (set `self.QuestDataNonRep` _questsinfo)
  (`KismetArrayLibrary.Array_Clear` _quests)
  (`KismetArrayLibrary.Array_Clear` _questsinfo)
  (return true))

(fn `OnRep_PlayerQuests`
  (bind _returnvalue (`self.GetOwner`))
  (bind _asplayer_controller (cast `PlayerController` _returnvalue))
  (if (`Controller.IsLocalController` _asplayer_controller)
    (bind _inv (message `/Game/RPG/Blueprints/Character/Interfaces/BP_ARPGControllerInterface.GetInventoryComponent` _returnvalue))
    (`/Game/RPG/Widgets/BP_MainInventory.RefreshQuests` (`/Game/RPG/Blueprints/InventorySystem/Components/BP_InventoryComponent.GetInventoryRef` _inv))))

(fn `QuestTrack_Currency`
  (params (Inv :type "/Game/RPG/Blueprints/InventorySystem/Components/BP_InventoryComponent Object Reference") (`CheckQuestStatus?` :type Boolean))
  (locals (CurrentGold :type "Float (double-precision)" :default 0.0))
  (set `local.CurrentGold` (`/Game/RPG/Blueprints/InventorySystem/Components/BP_InventoryComponent.GetTotalGoldInFloat` Inv (`/Game/RPG/Blueprints/InventorySystem/Components/BP_InventoryComponent.Credits` Inv) 0.0))
  (for (_array_element _array_index) (`self.PlayerQuests`)
    (bind ((`CurrentStatus_6_C0B23D5F427B94BC5FAB6C982F190F9E` _currentstatus) (`Objectives_13_7573456046651D48DA23EAA039CEFA45` _objectives)) (break `/Game/RPG/Blueprints/QuestSystem/QuestCreator/Data/S_PlayerQuestStatus` _array_element))
    (if (or (`|EnumEquality` _currentstatus "NewEnumerator0") (`|EnumEquality` _currentstatus "NewEnumerator2"))
      (for (_array_element_2 _array_index_2) _objectives
        (if (`|EnumEquality` (`.Type_2_88BA4D0B462FB1C99959DC93CF051C40` (break `/Game/RPG/Blueprints/QuestSystem/QuestCreator/Data/S_RepQuestObjective` _array_element_2)) "NewEnumerator4")
          (setmembers `/Game/RPG/Blueprints/QuestSystem/QuestCreator/Data/S_RepQuestObjective` :`StructRef` (`|GetArrayItem` (`.Objectives_13_7573456046651D48DA23EAA039CEFA45` (break `/Game/RPG/Blueprints/QuestSystem/QuestCreator/Data/S_PlayerQuestStatus` (`|GetArrayItem` (`self.PlayerQuests`) _array_index))) _array_index_2) :`CurrentCount` (`local.CurrentGold`))))))
  (if (`local.CheckQuestStatus?`)
    (`self.CheckForCompletedQuests`)))

(fn `QuestTrack_OnActorKilled`
  (params (ActorRef :type "Actor Object Reference"))
  (locals (Index :type Integer) (Index2 :type Integer) (`CheckForCompletion?` :type Boolean))
  ;[1 1 1] Actor killed, can be anything that gets destroyed
  (`/Engine/EditorBlueprintResources/StandardMacros.IsValid` ActorRef
    (:`Is Valid`
      (for (_array_element _array_index) (`self.PlayerQuests`)
        (set `local.Index` _array_index)
        (bind ((`CurrentStatus_6_C0B23D5F427B94BC5FAB6C982F190F9E` _currentstatus) (`Objectives_13_7573456046651D48DA23EAA039CEFA45` _objectives)) (break `/Game/RPG/Blueprints/QuestSystem/QuestCreator/Data/S_PlayerQuestStatus` _array_element))
        (if (`|EnumEquality` _currentstatus "NewEnumerator0")
          (for (_array_element_2 _array_index_2) _objectives
            (set `local.Index2` _array_index_2)
            (bind ((`Type_2_88BA4D0B462FB1C99959DC93CF051C40` _type) (`CurrentCount_20_D69E848B40B7E925F5C1FCA7F2CC1B9E` _currentcount) (`ObjectiveCount_21_4E02AFDD4BC542F68100068E434E6F04` _objectivecount)) (break `/Game/RPG/Blueprints/QuestSystem/QuestCreator/Data/S_RepQuestObjective` _array_element_2))
            (if (and (`|EnumEquality` _type "NewEnumerator0") (< _currentcount _objectivecount))
              (if (== (`.OfActorClass_9_F44F882B4D7C62F65D2C8CB2A00C89BC` (break `/Game/RPG/Blueprints/QuestSystem/QuestCreator/Data/S_QuestObjective` (`|GetArrayItem` (`.Objectives_26_348B948B4771E0192E317E911A007B98` (break `/Game/RPG/Blueprints/QuestSystem/QuestCreator/Data/S_QuestInfo` (`|GetArrayItem` (`self.QuestDataNonRep`) (`local.Index`)))) _array_index_2))) (`GameplayStatics.GetObjectClass` (`local.ActorRef`)))
                (`/Engine/EditorBlueprintResources/StandardMacros.IncrementFloat` (`.CurrentCount_20_D69E848B40B7E925F5C1FCA7F2CC1B9E` (break `/Game/RPG/Blueprints/QuestSystem/QuestCreator/Data/S_RepQuestObjective` (`|GetArrayItem` (`.Objectives_13_7573456046651D48DA23EAA039CEFA45` (break `/Game/RPG/Blueprints/QuestSystem/QuestCreator/Data/S_PlayerQuestStatus` (`|GetArrayItem` (`self.PlayerQuests`) (`local.Index`)))) (`local.Index2`))))
                  (:`  `
                    (set `local.CheckForCompletion?` true))))))))
      (if (`local.CheckForCompletion?`)
        (`self.CheckForCompletedQuests`)))))

(fn `QuestTrack_OnAreaReached`
  (params (`AreaName/Tag` :type Name))
  (locals (Index :type Integer) (Index2 :type Integer) (`CheckForCompletion?` :type Boolean))
  (bind ((`CurrentCount_20_D69E848B40B7E925F5C1FCA7F2CC1B9E` _currentcount) (`ObjectiveCount_21_4E02AFDD4BC542F68100068E434E6F04` _objectivecount)) (break `/Game/RPG/Blueprints/QuestSystem/QuestCreator/Data/S_RepQuestObjective` (`|GetArrayItem` (`.Objectives_13_7573456046651D48DA23EAA039CEFA45` (break `/Game/RPG/Blueprints/QuestSystem/QuestCreator/Data/S_PlayerQuestStatus` (`|GetArrayItem` (`self.PlayerQuests`) (`local.Index`)))) (`local.Index2`))))
  ;[1 1 1] You can call this function when the player reaches a certain area, you can pass the ID you entered in the quest objective
  (for (_array_element _array_index) (`self.PlayerQuests`)
    (set `local.Index` _array_index)
    (bind ((`CurrentStatus_6_C0B23D5F427B94BC5FAB6C982F190F9E` _currentstatus) (`Objectives_13_7573456046651D48DA23EAA039CEFA45` _objectives)) (break `/Game/RPG/Blueprints/QuestSystem/QuestCreator/Data/S_PlayerQuestStatus` _array_element))
    (if (`|EnumEquality` _currentstatus "NewEnumerator0")
      (for (_array_element_2 _array_index_2) _objectives
        (set `local.Index2` _array_index_2)
        (if (`|EnumEquality` (`.Type_2_88BA4D0B462FB1C99959DC93CF051C40` (break `/Game/RPG/Blueprints/QuestSystem/QuestCreator/Data/S_RepQuestObjective` _array_element_2)) "NewEnumerator3")
          (if (== (`.OrTagID_13_73AF88824DDC4605B8744094D5240D65` (break `/Game/RPG/Blueprints/QuestSystem/QuestCreator/Data/S_QuestObjective` (`|GetArrayItem` (`.Objectives_26_348B948B4771E0192E317E911A007B98` (break `/Game/RPG/Blueprints/QuestSystem/QuestCreator/Data/S_QuestInfo` (`|GetArrayItem` (`self.QuestDataNonRep`) (`local.Index`)))) (`local.Index2`)))) (`local.AreaName/Tag`))
            (if (< _currentcount _objectivecount)
              (`/Engine/EditorBlueprintResources/StandardMacros.IncrementFloat` _currentcount
                (:`  `
                  (set `local.CheckForCompletion?` true)))))))))
  (if (`local.CheckForCompletion?`)
    (`self.CheckForCompletedQuests`)))

(fn `QuestTrack_OnInteractedWith`
  (params (WithActor :type "Actor Object Reference"))
  (locals (Index :type Integer) (Index2 :type Integer) (`CheckForCompletion?` :type Boolean))
  (bind _withactor (`local.WithActor`))
  (bind ((`ActionName_22_FACA197844ED72BCE7D9539BC9F5ADCE` _actionname) (`OfActorClass_9_F44F882B4D7C62F65D2C8CB2A00C89BC` _ofactorclass) (`OrTagID_13_73AF88824DDC4605B8744094D5240D65` _ortagid)) (break `/Game/RPG/Blueprints/QuestSystem/QuestCreator/Data/S_QuestObjective` (`|GetArrayItem` (`.Objectives_26_348B948B4771E0192E317E911A007B98` (break `/Game/RPG/Blueprints/QuestSystem/QuestCreator/Data/S_QuestInfo` (`|GetArrayItem` (`self.QuestDataNonRep`) (`local.Index`)))) (`local.Index2`))))
  (bind ((`CurrentCount_20_D69E848B40B7E925F5C1FCA7F2CC1B9E` _currentcount) (`ObjectiveCount_21_4E02AFDD4BC542F68100068E434E6F04` _objectivecount)) (break `/Game/RPG/Blueprints/QuestSystem/QuestCreator/Data/S_RepQuestObjective` (`|GetArrayItem` (`.Objectives_13_7573456046651D48DA23EAA039CEFA45` (break `/Game/RPG/Blueprints/QuestSystem/QuestCreator/Data/S_PlayerQuestStatus` (`|GetArrayItem` (`self.PlayerQuests`) (`local.Index`)))) (`local.Index2`))))
  (`/Engine/EditorBlueprintResources/StandardMacros.IsValid` WithActor
    (:`Is Valid`
      (for (_array_element _array_index) (`self.PlayerQuests`)
        (set `local.Index` _array_index)
        (bind ((`CurrentStatus_6_C0B23D5F427B94BC5FAB6C982F190F9E` _currentstatus) (`Objectives_13_7573456046651D48DA23EAA039CEFA45` _objectives)) (break `/Game/RPG/Blueprints/QuestSystem/QuestCreator/Data/S_PlayerQuestStatus` _array_element))
        (if (`|EnumEquality` _currentstatus "NewEnumerator0")
          (for (_array_element_2 _array_index_2) _objectives
            (set `local.Index2` _array_index_2)
            (if (`|EnumEquality` (`.Type_2_88BA4D0B462FB1C99959DC93CF051C40` (break `/Game/RPG/Blueprints/QuestSystem/QuestCreator/Data/S_RepQuestObjective` _array_element_2)) "NewEnumerator2")
              (if (or (== _ofactorclass (`GameplayStatics.GetObjectClass` _withactor)) (and (not (`KismetSystemLibrary.IsValidClass` _ofactorclass)) (`KismetArrayLibrary.Array_Contains` (`Actor.Tags` _withactor) _ortagid)))
                (if (< _currentcount _objectivecount)
                  (`/Engine/EditorBlueprintResources/StandardMacros.IncrementFloat` _currentcount
                    (:`  `
                      (set `local.CheckForCompletion?` true)))))))))
      (if (`local.CheckForCompletion?`)
        (`self.CheckForCompletedQuests`)))))

(fn `QuestTrack_OnInventoryItemsUpdated`
  (params (CheckGold :type Boolean))
  (locals (ItemIDs :type "Array of Name") (Index1 :type "Array of Integer") (Index2 :type "Array of Integer") (CurrentID :type Name))
  (bind _inv (message `/Game/RPG/Blueprints/Character/Interfaces/BP_ARPGControllerInterface.GetInventoryComponent` (`self.GetOwner`)))
  (`/Engine/EditorBlueprintResources/StandardMacros.IsValid` _inv
    (:`Is Valid`
      (if (`local.CheckGold`)
        (`self.QuestTrack_Currency` _inv))
      (`|ExecutionSequence`
        (:`then_0`
          (for (_array_element _array_index) (`self.PlayerQuests`)
            (bind ((`CurrentStatus_6_C0B23D5F427B94BC5FAB6C982F190F9E` _currentstatus) (`Objectives_13_7573456046651D48DA23EAA039CEFA45` _objectives)) (break `/Game/RPG/Blueprints/QuestSystem/QuestCreator/Data/S_PlayerQuestStatus` _array_element))
            (if (or (`|EnumEquality` _currentstatus "NewEnumerator0") (`|EnumEquality` _currentstatus "NewEnumerator2"))
              (for (_array_element_2 _array_index_2) _objectives
                (if (`|EnumEquality` (`.Type_2_88BA4D0B462FB1C99959DC93CF051C40` (break `/Game/RPG/Blueprints/QuestSystem/QuestCreator/Data/S_RepQuestObjective` _array_element_2)) "NewEnumerator1")
                  (`KismetArrayLibrary.Array_AddUnique` (`local.ItemIDs`) (`.OrTagID_13_73AF88824DDC4605B8744094D5240D65` (break `/Game/RPG/Blueprints/QuestSystem/QuestCreator/Data/S_QuestObjective` (`|GetArrayItem` (`.Objectives_26_348B948B4771E0192E317E911A007B98` (break `/Game/RPG/Blueprints/QuestSystem/QuestCreator/Data/S_QuestInfo` (`|GetArrayItem` (`self.QuestDataNonRep`) _array_index))) _array_index_2))))
                  (`KismetArrayLibrary.Array_Add` (`local.Index1`) _array_index)
                  (`KismetArrayLibrary.Array_Add` (`local.Index2`) _array_index_2))))))
        (:`then_1`
          (if (`KismetArrayLibrary.Array_IsValidIndex` (`local.ItemIDs`))
            (bind _result (`/Game/RPG/Blueprints/InventorySystem/Components/BP_InventoryComponent.GetCountOfInventoryItems` _inv (`local.ItemIDs`)))
            (for (_array_element_3 _array_index_3) (`local.Index1`)
              (bind _output (`|GetArrayItem` (`local.Index2`) _array_index_3))
              (set `local.CurrentID` (`.OrTagID_13_73AF88824DDC4605B8744094D5240D65` (break `/Game/RPG/Blueprints/QuestSystem/QuestCreator/Data/S_QuestObjective` (`|GetArrayItem` (`.Objectives_26_348B948B4771E0192E317E911A007B98` (break `/Game/RPG/Blueprints/QuestSystem/QuestCreator/Data/S_QuestInfo` (`|GetArrayItem` (`self.QuestDataNonRep`) _array_element_3))) _output))))
              (setmembers `/Game/RPG/Blueprints/QuestSystem/QuestCreator/Data/S_RepQuestObjective` :`StructRef` (`|GetArrayItem` (`.Objectives_13_7573456046651D48DA23EAA039CEFA45` (break `/Game/RPG/Blueprints/QuestSystem/QuestCreator/Data/S_PlayerQuestStatus` (`|GetArrayItem` (`self.PlayerQuests`) _array_element_3))) _output) :`CurrentCount` (`KismetMathLibrary.Conv_IntToDouble` (`BlueprintMapLibrary.Map_Find` _result (`local.CurrentID`)))))
            (`self.CheckForCompletedQuests`)))))))

(fn `SaveQuests`
  (params (SaveDataRef :type "/Game/RPG/Blueprints/InventorySystem/SaveSystem/SaveData Structure (by ref)"))
  (returns (Result :type Boolean))
  (setmembers `/Game/RPG/Blueprints/InventorySystem/SaveSystem/SaveData` :`StructRef` SaveDataRef :`Quests` (`self.PlayerQuests`) :`QuestsInfo` (`self.QuestDataNonRep`))
  (return true))

(fn `SetQuestStatusByID`
  (params (QuestUID :type Name) (CurrentStatus :type "/Game/RPG/Blueprints/QuestSystem/QuestCreator/Data/E_QuestStatus Enum" :default "NewEnumerator0") (CurrentProgressUID :type Integer))
  (for (_array_element _array_index) (`self.PlayerQuests`)
    (if (== (`.UniqueQuestID_3_12E1AFAE40DEF67DD7A4F8A2397E8304` (break `/Game/RPG/Blueprints/QuestSystem/QuestCreator/Data/S_PlayerQuestStatus` _array_element)) (`local.QuestUID`))
      (setmembers `/Game/RPG/Blueprints/QuestSystem/QuestCreator/Data/S_PlayerQuestStatus` :`StructRef` (`|GetArrayItem` (`self.PlayerQuests`) _array_index) :`CurrentStatus` (`local.CurrentStatus`) :`CurrentProgressUID` (`local.CurrentProgressUID`))
      (return)))
  (return))