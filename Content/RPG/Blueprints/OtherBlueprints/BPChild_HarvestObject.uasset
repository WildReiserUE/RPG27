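; Harvestable interactable child Blueprint that runs a random spawner when a character interacts with it.
; Clients forward the interaction through a server request on the passed component, while the authority processes it once, gated by the spawner condition.
; One of the two accepted conditions also reports earned experience to the character and destroys the actor.
; The outline override calls the parent, then drives the static mesh's custom depth rendering.
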(event `/Game/RPG/Blueprints/Interfaces/IT_InteractInterface.ExecuteInteract`
  (params (CharacterRef :type "Actor Object Reference") (Comp :type "/Game/RPG/Blueprints/Components/BP_AC_General Object Reference"))
  (bind _spawnercondition (`self.SpawnerCondition`))
  (bind _returnvalue (`|EnumEquality` _spawnercondition "NewEnumerator1"))
  ;[0.04688 0.04688 0.04688] Spawn on interact
  (if (`self.HasAuthority` CharacterRef)
    (`/Engine/EditorBlueprintResources/StandardMacros.DoOnce` false
      (:`Completed`
        (if (or _returnvalue (`|EnumEquality` _spawnercondition "NewEnumerator2"))
          (`self.ProcessRandomSpawner`)
          (if _returnvalue
            (message `/Game/RPG/Blueprints/Interfaces/IT_SkillEffects.Skill_OnTargetExpEarned` CharacterRef self (`self.ExpEarned`) false)
            (`self.K2_DestroyActor`)))))
    (else
      (`/Game/RPG/Blueprints/Components/BP_AC_General.SERVER_RequestInteractWithActor` Comp self))))

(fn `SetOutlineEnabled`
  (params (Enabled :type Boolean) (InteractKey :type "Key Structure") (CalledFrom :type "Actor Object Reference"))
  (returns (`Enabled?` :type Boolean))
  (bind _outlineon (`self.OutlineOn`))
  (`parent.SetOutlineEnabled` Enabled InteractKey null)
  (`PrimitiveComponent.SetRenderCustomDepth` (`self.StaticMesh`) _outlineon)
  (return _outlineon))

(fn `UserConstructionScript`
  (`parent.UserConstructionScript`))