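; BP_Respawner is a temporary server-side actor that respawns a harvesting actor after a random delay within its RespawnTime range.
; It box-traces its stored bounds for Pawns and, while blocked, retries every few seconds, destroying itself once the attempt limit is exceeded.
; When clear, it spawns ActorClassToSpawn, passing along the stored spawner, pickup, health and interaction settings, then destroys itself on success or retries on failure.
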(event `AttemptSpawn`
  ;[0.04167 0.04167 0.04167] Respawn harvesting BP
  (if (`self.CheckCollision`) :!label _label
    (if (> (`self.SpawnAttempts`) 99) :!label _label_2
      (`self.K2_DestroyActor` :!label _label_3)
      (else
        (`/Engine/EditorBlueprintResources/StandardMacros.IncrementInt` (`self.SpawnAttempts`)
          (:`  `
            (`KismetSystemLibrary.Delay` 5.0)
            (`self.AttemptSpawn`)))))
    (else
      (bind _returnvalue (`|SpawnActorFromClass` (`self.ActorClassToSpawn`) (`self.SpawnT`) "AlwaysSpawn" "OverrideRootScale" null (`self.Show Name Widget?`) (`self.Spawner Name`) (`self.Spawner Name Color`) (`self.Possible Spawn Pickups`) (`self.Spawner Condition`) (`self.Health`) (`self.Max Damage Per Hit`) (`self.Max Random Spawn Distance`) (`self.Apply Inpulse?`) (`self.XYInpulse`) (`self.ZInpulse`) (`self.Max Items to Spawn`) (`self.RespawnTime`) (`self.Required Duration for Interaction`) (`self.Exp Earned`) null))
      (`/Engine/EditorBlueprintResources/StandardMacros.IsValid` _returnvalue
        (:`Is Valid`
          (goto _label_3))
        (:`Is Not Valid`
          (goto _label_2))))))

(event `self.ReceiveBeginPlay`
  (bind (_respawntime_x _respawntime_y) (`KismetMathLibrary.BreakVector2D` (`self.RespawnTime`)))
  ;[0.04167 0.04167 0.04167] Respawn harvesting BP
  (`/Engine/EditorBlueprintResources/ActorMacros.Switch Has Authority`
    (:`Authority`
      (bind _output_get (set `self.dur` (`KismetMathLibrary.RandomFloatInRange` _respawntime_x _respawntime_y)))
      (`KismetSystemLibrary.Delay` _output_get)
      (goto _label))))

(fn `CheckCollision`
  (returns (ReturnValue :type Boolean))
  (bind _boundorigin (`self.BoundOrigin`))
  (bind (_outhit _returnvalue) (`KismetSystemLibrary.BoxTraceSingleForObjects` _boundorigin _boundorigin (`self.BoundExtent`) (struct) (`|MakeArray` "ObjectTypeQuery3" :!type "EObjectTypeQuery Enum")))
  (return _returnvalue))

(fn `UserConstructionScript`)