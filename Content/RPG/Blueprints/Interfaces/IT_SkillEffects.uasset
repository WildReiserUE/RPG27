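; Blueprint interface for actors that take part in the RPG skill and effect system.
; It declares callbacks for effects starting, expiring, being added, removed or refreshed, identified by a unique ID, plus notifications for target damage and earned experience.
; Query functions report alive, stunned and skill-performing states, capsule size and duel target, alongside a setter for the duel target.
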(fn `Skill_GetCapsuleSize`
  (returns (Height :type "Float (double-precision)") (Radius :type "Float (double-precision)"))
  (return 0.0 0.0))

(fn `Skill_HasDuelTarget`
  (returns (Result :type Boolean) (DuelTarget :type "Actor Object Reference"))
  (return false null))

(fn `Skill_IsAlive`
  (returns (Result :type Boolean))
  (return false))

(fn `Skill_IsPerformingSkill`
  (returns (Result :type Boolean) (CurrentSkill :type "/Game/RPG/Blueprints/Skills/Data/S_SkillInfo Structure"))
  (return false))

(fn `Skill_IsStunned?`
  (returns (Result :type Boolean))
  (return false))

(fn `Skill_OnEffectAdded`
  (params (Effect :type "/Game/RPG/Blueprints/Skills/Data/S_SkillEffects Structure") (UniqueID :type Integer))
  (returns (Result :type Boolean))
  (return false))

(fn `Skill_OnEffectRefreshed`
  (params (Effect :type "/Game/RPG/Blueprints/Skills/Data/S_SkillEffects Structure") (UniqueID :type Integer))
  (returns (Result :type Boolean))
  (return false))

(fn `Skill_OnEffectRemoved`
  (params (Effect :type "/Game/RPG/Blueprints/Skills/Data/S_SkillEffects Structure") (UniqueID :type Integer))
  (returns (Result :type Boolean))
  (return false))

(fn `Skill_OnEffectsEndDuration`
  (params (Effect :type "/Game/RPG/Blueprints/Skills/Data/S_SkillEffects Structure") (Causer :type "Actor Object Reference") (UniqueID :type Integer))
  (returns (Result :type Boolean))
  (return false))

(fn `Skill_OnEffectsStarted`
  (params (Effect :type "/Game/RPG/Blueprints/Skills/Data/S_SkillEffects Structure") (Causer :type "Actor Object Reference") (`AppliedOnce?` :type Boolean) (UniqueID :type Integer))
  (returns (Result :type Boolean))
  (return false))

(fn `Skill_OnTargetDamaged`
  (params (ActorDamaged :type "Actor Object Reference") (DamageApplied :type "Float (double-precision)") (TargetKilled :type Boolean))
  (returns (Result :type Boolean))
  (return false))

(fn `Skill_OnTargetExpEarned`
  (params (FromActor :type "Actor Object Reference") (Bounty :type "Float (double-precision)" :default 0.0) (IsSharedExp :type Boolean))
  (returns (Result :type Boolean))
  (return false))

(fn `Skill_SetDuelTarget`
  (params (PawnRef :type "Actor Object Reference"))
  (returns (Result :type Boolean))
  (return false))