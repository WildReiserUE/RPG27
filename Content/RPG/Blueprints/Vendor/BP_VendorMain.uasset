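; Vendor NPC that players interact with to open a shop of purchasable items.
; Interacting calls ShowVendor on the passed component; ShowContent lazily creates and caches a vendor widget, fills it from VendorItems with an optional inventory grid, and adds it through the inventory component.
; Modular armor meshes follow the body via master pose.
; A name widget shows the vendor name and interact key, while custom depth draws the highlight outline.
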(event `self.ReceiveBeginPlay`
  (bind _returnvalue (`WidgetComponent.GetUserWidgetObject` (`self.Widget`)))
  ;[1 1 1] Set character name
  (`/Engine/EditorBlueprintResources/StandardMacros.IsValid` _returnvalue
    (:`Is Valid`
      (bind _asbp_display_name (cast `/Game/RPG/Blueprints/InventorySystem/JigSaw/Widgets/BP_DisplayName` _returnvalue))
      (`/Game/RPG/Blueprints/InventorySystem/JigSaw/Widgets/BP_DisplayName.UpdateName` _asbp_display_name (`self.VendorName`) (struct :`R` 1.0 :`G` 1.0 :`B` 1.0 :`A` 1.0)))))

(event `/Game/RPG/Blueprints/Interfaces/BPI_Interact.ExecuteInteract`
  (params (CharacterRef :type "Actor Object Reference") (Comp :type "/Game/RPG/Blueprints/Components/BP_AC_General Object Reference"))
  ;[1 1 1] When interacted with
  (`/Game/RPG/Blueprints/Components/BP_AC_General.ShowVendor` Comp self))

(fn `CanBeDamagedByPlayer?`
  (returns (Result :type Boolean))
  (return false))

(fn `CanInteract?`
  (returns (Result :type Boolean) (RequiredDuration :type "Float (double-precision)"))
  (return true 0.0))

(fn `GetAcceptableDistance`
  (returns (Distance :type "Float (double-precision)"))
  (return 100.0))

(fn `GetActorName`
  (returns (PlayerName :type String))
  (return ""))

(fn `GetAIBehavior`
  (returns (Behavior :type "/Game/RPG/Blueprints/AI/Data/E_AIBehaviorType Enum"))
  (return "NewEnumerator3"))

(fn `GetAIHostility`
  (returns (Result :type "/Game/RPG/Blueprints/AI/Data/E_AIHostilityType Enum"))
  (return "NewEnumerator3"))

(fn `GetBountyExp`
  (returns (Exp :type "Float (double-precision)"))
  (return 0.0))

(fn `GetOutlineColor`
  (returns (Color :type "LinearColor Structure"))
  (return (struct :`G` 0.738189 :`B` 1.0 :`A` 1.0)))

(fn `IsWVisible`
  (returns (ReturnValue :type Boolean))
  ;[1 1 1] Checks if vendor widget is visibe
  (return (`Widget.IsVisible` (`self.VendorWidgetRef`))))

(fn `OnBeginInteract`
  (returns (Result :type Boolean))
  (return false))

(fn `OnEndInteract`
  (returns (Result :type Boolean))
  (return false))

(fn `SetHostility`
  (params (NewHostility :type "/Game/RPG/Blueprints/AI/Data/E_AIHostilityType Enum" :default "NewEnumerator3"))
  (returns (Result :type Boolean))
  (return false))

(fn `SetHostilityColor`
  (params (IsHostile :type Boolean) (`IsParty?` :type Boolean) (`IsGuild?` :type Boolean))
  (returns (Result :type Boolean))
  (return false))

(fn `SetOutlineEnabled`
  (params (Enabled :type Boolean) (InteractKey :type "Key Structure") (CalledFrom :type "Actor Object Reference"))
  (returns (`Enabled?` :type Boolean))
  (locals (NoneKey :type "Key Structure" :default "None"))
  (bind _returnvalue (== InteractKey (`local.NoneKey`)))
  ;[1 1 1] Sets the outline, the key is used in third person mode
  (bind _output_get (set `/Game/RPG/Blueprints/Components/BP_NameVisibility.OutlineOn` Enabled (`self.BP_NameVisibility`)))
  (`PrimitiveComponent.SetRenderCustomDepth` (`self.Mesh`) _output_get)
  (`PrimitiveComponent.SetRenderCustomDepth` (`self.Helmet`) _output_get)
  (`PrimitiveComponent.SetRenderCustomDepth` (`self.Pants`) _output_get)
  (`PrimitiveComponent.SetRenderCustomDepth` (`self.Gloves`) _output_get)
  (`PrimitiveComponent.SetRenderCustomDepth` (`self.Belt`) _output_get)
  (`PrimitiveComponent.SetRenderCustomDepth` (`self.Shoulder`) _output_get)
  (`PrimitiveComponent.SetRenderCustomDepth` (`self.Boots`) _output_get)
  (`|ExecutionSequence`
    (:`then_0`
      (if (not _returnvalue)
        (bind _asbp_display_name (cast `/Game/RPG/Blueprints/InventorySystem/JigSaw/Widgets/BP_DisplayName` (`WidgetComponent.GetUserWidgetObject` (`self.Widget`))))
        (`/Game/RPG/Blueprints/InventorySystem/JigSaw/Widgets/BP_DisplayName.SetInteractKey` _asbp_display_name (`KismetInputLibrary.Key_GetDisplayName` InteractKey) (or _returnvalue (not _output_get)))))
    (:`then_1`
      (return Enabled))))

(fn `ShowContent`
  (params (InvComponent :type "/Game/RPG/Blueprints/Components/BP_AC_General Object Reference"))
  (bind _vendorwidgetref (`self.VendorWidgetRef`))
  ;[1 1 1] Creates the vendor widget then use the settings to add the items that are available for purchase, then add the item to the viewport
  (`|ExecutionSequence`
    (:`then_0`
      (`/Engine/EditorBlueprintResources/StandardMacros.IsValid` (`self.VendorWidgetRef`)
        (:`Is Not Valid`
          (bind _returnvalue (`|CreateWidget` "/Game/RPG/Blueprints/Vendor/Widgets/BP_VendorWidget.BP_VendorWidget_C"))
          (bind _output_get (set `self.VendorWidgetRef` _returnvalue))
          (set `/Game/RPG/Blueprints/Vendor/Widgets/BP_VendorWidget.InvComponent` (`local.InvComponent`) (`self.VendorWidgetRef`))
          (set `/Game/RPG/Blueprints/Vendor/Widgets/BP_VendorWidget.VendorRef` self _output_get)
          (`/Game/RPG/Blueprints/Vendor/Widgets/BP_VendorWidget.SetVendorName` _output_get (`self.VendorName`))
          (`|ExecutionSequence`
            (:`then_0`
              (if (`self.UseFullInventory?`)
                (`/Game/RPG/Blueprints/Vendor/Widgets/BP_VendorWidget.CreateFullInventory` (`self.VendorWidgetRef`) (`self.FullInventory_Rows`) (`self.FullInventory_Columns`))))
            (:`then_1`
              (for _array_element (`self.VendorItems`)
                (bind (_itemid _indatatable _price _customimage) (break `/Game/RPG/Blueprints/Vendor/Data/VendorItems` _array_element))
                (`/Game/RPG/Blueprints/Vendor/Widgets/BP_VendorWidget.AddNewItem` (`self.VendorWidgetRef`) _itemid _indatatable _price _customimage)))))))
    (:`then_1`
      (if (not (`Widget.IsVisible` _vendorwidgetref))
        (`/Game/RPG/Blueprints/Components/BP_AC_General.AddContent` InvComponent _vendorwidgetref)))))

(fn `UserConstructionScript`
  (`SkinnedMeshComponent.SetLeaderPoseComponent` (`self.Armor`) (`self.Mesh`) false)
  (`SkinnedMeshComponent.SetLeaderPoseComponent` (`self.Helmet`) (`self.Mesh`) false)
  (`SkinnedMeshComponent.SetLeaderPoseComponent` (`self.Boots`) (`self.Mesh`) false)
  (`SkinnedMeshComponent.SetLeaderPoseComponent` (`self.Pants`) (`self.Mesh`) false)
  (`SkinnedMeshComponent.SetLeaderPoseComponent` (`self.Gloves`) (`self.Mesh`) false)
  (`SkinnedMeshComponent.SetLeaderPoseComponent` (`self.Belt`) (`self.Mesh`) false)
  (`SkinnedMeshComponent.SetLeaderPoseComponent` (`self.Shoulder`) (`self.Mesh`) false)
  (set `/Game/RPG/Blueprints/Components/BP_NameVisibility.Widget` (`self.Widget`) (`self.BP_NameVisibility`)))