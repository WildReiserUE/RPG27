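; BP_Skill_Arrow is an arrow skill actor that damages the first valid hostile it overlaps.
; On construction it moves just in front of its owning pawn and slightly up, rotating toward the skill target if one exists.
; On sphere overlap, the server checks the target is damageable, hostile and alive, then applies damage, notifies the owner, applies skill effects and destroys the arrow.
; Any hit also destroys it.
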(event `self.ReceiveBeginPlay`
  (`parent.ReceiveBeginPlay`))

(event `self.Sphere.OnComponentBeginOverlap`
  (params (OverlappedComponent :type "PrimitiveComponent Object Reference") (OtherActor :type "Actor Object Reference") (OtherComp :type "PrimitiveComponent Object Reference") (OtherBodyIndex :type Integer) (bFromSweep :type Boolean) (SweepResult :type "HitResult Structure (by ref)"))
  (if (!= OtherActor (`self.PawnOwner`))
    (`/Engine/EditorBlueprintResources/ActorMacros.Switch Has Authority`
      (:`Authority`
        (if (and (`Actor.bCanBeDamaged` OtherActor) (`self.IsTargetHostile` OtherActor) (`self.IsTargetAlive?` OtherActor))
          (bind _returnvalue (`GameplayStatics.ApplyDamage` OtherActor (`self.SkillDamage`) null (`self.PawnOwner`) (`self.DamageType`)))
          (message `/Game/RPG/Blueprints/Skills/Blueprint/SkillComponent/IT_SkillEffects.Skill_OnTargetDamaged` (`self.PawnOwner`) OtherActor _returnvalue false)
          (`self.ApplySkillEffects` OtherActor)
          (`self.K2_DestroyActor`))))))

(event `self.ReceiveHit`
  (params (MyComp :type "PrimitiveComponent Object Reference") (Other :type "Actor Object Reference") (OtherComp :type "PrimitiveComponent Object Reference") (bSelfMoved :type Boolean) (HitLocation :type "Vector Structure") (HitNormal :type "Vector Structure") (NormalImpulse :type "Vector Structure") (Hit :type "HitResult Structure (by ref)"))
  (`self.K2_DestroyActor`))

(fn `UserConstructionScript`
  (bind _pawnowner (`self.PawnOwner`))
  (`parent.UserConstructionScript`)
  (`/Engine/EditorBlueprintResources/StandardMacros.IsValid` (`self.PawnOwner`)
    (:`Is Valid`
      (`/Engine/EditorBlueprintResources/StandardMacros.IsValid` (`self.SkillTarget`)
        (:`Is Valid`
          (`self.K2_SetActorRotation` (`KismetMathLibrary.FindLookAtRotation` (`self.K2_GetActorLocation`) (`self.K2_GetActorLocation` (`self.SkillTarget`))) true))
        (:`Is Not Valid`
          (`self.K2_SetActorRotation` (`self.K2_GetActorRotation`) true)))
      (`self.K2_SetActorLocation` (+ (`self.K2_GetActorLocation` _pawnowner) (* (`self.GetActorForwardVector` _pawnowner) 75.0) (0.0 0.0 25.0)) false true))))