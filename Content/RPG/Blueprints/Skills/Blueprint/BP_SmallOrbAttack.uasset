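; Small homing orb skill projectile that spawns just in front of its PawnOwner, tinted red through a dynamic material.
; Each tick it rotates toward a live, hostile SkillTarget and resets its velocity to a fixed forward speed.
; On the server, overlapping a damageable, live hostile deals skill damage, notifies the owner, applies skill effects and destroys the orb, while a Hit event simply destroys it.
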(event `self.Sphere.OnComponentBeginOverlap`
  (params (OverlappedComponent :type "PrimitiveComponent Object Reference") (OtherActor :type "Actor Object Reference") (OtherComp :type "PrimitiveComponent Object Reference") (OtherBodyIndex :type Integer) (bFromSweep :type Boolean) (SweepResult :type "HitResult Structure (by ref)"))
  (if (!= OtherActor (`self.PawnOwner`))
    (`/Engine/EditorBlueprintResources/ActorMacros.Switch Has Authority`
      (:`Authority`
        (if (and (`Actor.bCanBeDamaged` OtherActor) (`self.IsTargetHostile` OtherActor) (`self.IsTargetAlive?` OtherActor))
          (bind _returnvalue (`GameplayStatics.ApplyDamage` OtherActor (`self.SkillDamage`) null (`self.PawnOwner`) (`self.DamageType`)))
          (message `/Game/RPG/Blueprints/Interfaces/IT_SkillEffects.Skill_OnTargetDamaged` (`self.PawnOwner`) OtherActor _returnvalue false)
          (`self.ApplySkillEffects` OtherActor)
          (`self.K2_DestroyActor`))))))

(event `self.ReceiveHit`
  (params (MyComp :type "PrimitiveComponent Object Reference") (Other :type "Actor Object Reference") (OtherComp :type "PrimitiveComponent Object Reference") (bSelfMoved :type Boolean) (HitLocation :type "Vector Structure") (HitNormal :type "Vector Structure") (NormalImpulse :type "Vector Structure") (Hit :type "HitResult Structure (by ref)"))
  (`/Engine/EditorBlueprintResources/ActorMacros.Switch Has Authority`
    (:`Authority`
      (`self.K2_DestroyActor`))))

(event `self.ReceiveTick`
  (params (DeltaSeconds :type "Float (single-precision)"))
  (bind _skilltarget (`self.SkillTarget`))
  ;[1 1 1] Track target
  (`parent.ReceiveTick` DeltaSeconds)
  (`/Engine/EditorBlueprintResources/StandardMacros.IsValid` _skilltarget
    (:`Is Valid`
      (if (and (`self.IsTargetAlive?` _skilltarget) (`self.IsTargetHostile` _skilltarget))
        (`self.K2_SetActorRotation` (`KismetMathLibrary.FindLookAtRotation` (`self.K2_GetActorLocation`) (`self.K2_GetActorLocation` (`self.SkillTarget`))) true)
        (set `MovementComponent.Velocity` (* (`self.GetActorForwardVector`) 1000.0) (`self.ProjectileMovement`))))))

(fn `UserConstructionScript`
  (bind _pawnowner (`self.PawnOwner`))
  (`parent.UserConstructionScript`)
  (bind _returnvalue (`PrimitiveComponent.CreateDynamicMaterialInstance` (`self.Sphere_0`) 0 (`PrimitiveComponent.GetMaterial` (`self.Sphere_0`) 0) "None"))
  (`MaterialInstanceDynamic.SetVectorParameterValue` _returnvalue "Color" (struct :`R` 1.0 :`A` 1.0))
  (`/Engine/EditorBlueprintResources/StandardMacros.IsValid` (`self.PawnOwner`)
    (:`Is Valid`
      (`self.K2_SetActorLocation` (+ (`self.K2_GetActorLocation` _pawnowner) (* (`self.GetActorForwardVector` _pawnowner) 50.0) (0.0 0.0 5.0)) false true))))