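; Crafting widget component that opens a crafting UI listing its configured AvailableCraftItems.
; ShowWidget creates BP_CraftingWidget on first use, sets the craft name and adds each item from its data table reference, passing along the random-stats option.
; Later calls reuse the cached widget and update its inventory component.
; If hidden, the widget refreshes its resource totals and is added as content through that inventory component.
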(fn `ShowWidget`
  (params (Name :type Text) (InvComponent :type "/Game/RPG/Blueprints/Components/BP_InventoryComponent Object Reference") (`RandomStats?` :type Boolean))
  ;[1 1 1] Initialize the crafting widget by adding the items from the settings then add the widget to the viewport
  (set `self.InvComponent` InvComponent)
  (`|ExecutionSequence`
    (:`then_0`
      (`/Engine/EditorBlueprintResources/StandardMacros.IsValid` (`self.WidgetRef`)
        (:`Is Not Valid`
          (bind _returnvalue (`|CreateWidget` "/Game/RPG/Blueprints/Crafting/Widgets/BP_CraftingWidget.BP_CraftingWidget_C"))
          (bind _output_get (set `self.WidgetRef` _returnvalue))
          (set `/Game/RPG/Blueprints/Crafting/Widgets/BP_CraftingWidget.InvComponent` (`self.InvComponent`) _output_get)
          (`/Game/RPG/Blueprints/Crafting/Widgets/BP_CraftingWidget.SetCraftName` _output_get (`local.Name`))
          (for _array_element (`self.AvailableCraftItems`)
            (bind (_itemid _indatatable _customimage) (break `/Game/RPG/Blueprints/Crafting/Data/CraftingItems` _array_element))
            (`/Game/RPG/Blueprints/Crafting/Widgets/BP_CraftingWidget.AddNewItem` :`self` (`self.WidgetRef`) :`ItemID` _itemid :`InDataTable` _indatatable :`CustomImage` _customimage :`RandomStats?` (`local.RandomStats?`))))))
    (:`then_1`
      (set `/Game/RPG/Blueprints/Crafting/Widgets/BP_CraftingWidget.InvComponent` (`self.InvComponent`) (`self.WidgetRef`))
      (if (not (`Widget.IsVisible` (`self.WidgetRef`)))
        (`/Game/RPG/Blueprints/Crafting/Widgets/BP_CraftingWidget.GetTotalResources` (`self.WidgetRef`))
        (`/Game/RPG/Blueprints/Components/BP_InventoryComponent.AddContent` (`local.InvComponent`) (`self.WidgetRef`))))))