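; Component managing a player's class skill tree: point allocation, resets, save data and the tree widget.
; The server enables skills in per-class config and applies passive stats through the item-equip message; client RPCs update the widget.
; Support passives roll trigger chances to append damage, slow, stun or knock effects to skills, then roll again to boost effect duration, damage and movement modifiers.
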(event `Initialize`
  (params (PlayerClass :type "/Game/RPG/Blueprints/InventorySystem/JigSaw/Data/E_ClassTypes Enum" :default "NewEnumerator0"))
  ;[0.07812 0.07812 0.07812] Create skill tree widget
  (set `self.PlayerClass` PlayerClass)
  (bind _returnvalue (`|CreateWidget` (`self.GetTreeWidgetByClass` PlayerClass)))
  (bind _output_get (set `self.TreeWidgetRef` _returnvalue))
  (message `/Game/RPG/Blueprints/Interfaces/BPI_SkillTree.SkillTree_SetSkillPoints` _output_get (`self.CurrentSkillPoints`) false))

(event `SERVER_AllocateSkillPoints`
  (params (SkillUniqueIDs :type "Array of Name"))
  ;[1 1 1] RPCs
  (`self.HandleAllocatingSkillPoints` SkillUniqueIDs))

(event `CLIENT_OnSkillPointsReset`
  (params (Points :type Integer))
  ;[1 1 1] Reset skill points
  (message `/Game/RPG/Blueprints/Interfaces/BPI_SkillTree.SkillTree_ResetPoints` (`self.GetTreeWidget`) Points)
  (bind _inv (message `/Game/RPG/Blueprints/Interfaces/BPI_Controller.GetInventoryComponent` (`GameplayStatics.GetPlayerController` 0)))
  (`/Game/RPG/Widgets/W_GameMain.ClearActionbars` (`/Game/RPG/Blueprints/Components/BP_AC_General.InGameWidgetRef` _inv)))

(event `CLIENT_SetActiveTreeSkills`
  (params (SkillUIDs :type "Array of Name") (AvailablePoints :type Integer))
  ;[1 1 1] RPCs
  (message `/Game/RPG/Blueprints/Interfaces/BPI_SkillTree.SkillTree_SetActiveSkills` (`self.GetTreeWidget`) SkillUIDs AvailablePoints))

(event `SetSkillPoints`
  (params (Points :type Integer))
  ;[1 1 1] RPCs
  (message `/Game/RPG/Blueprints/Interfaces/BPI_SkillTree.SkillTree_SetSkillPoints` (`self.GetTreeWidget`) Points true))

(event `CLIENT_OnSkillPointsEarned`
  (params (Points :type Integer))
  ;[1 1 1] RPCs
  (`self.SetSkillPoints` Points))

(fn `ApplyPassivesToSkillEffect`
  (params (Effects :type "Array of /Game/RPG/Blueprints/Skills/Data/S_SkillEffects Structure (by ref)") (Passives :type "Array of /Game/RPG/Blueprints/Skills/Data/S_PassiveSkillSettings Structure (by ref)") (SupportedSkill :type Name))
  (returns (Result :type "Array of /Game/RPG/Blueprints/Skills/Data/S_SkillEffects Structure (by ref)"))
  (locals (NewEffects :type "Array of /Game/RPG/Blueprints/Skills/Data/S_SkillEffects Structure") (Support :type "/Game/RPG/Blueprints/Skills/Data/S_PassiveSkillSettings Structure"))
  (bind ((`NewAddedEffectInterval_72_ED90BC2940A78CFC4E9D5E90B9DD95C1` _newaddedeffectinterval) (`NewAddedEffectDuration_73_3872F84042C7C0283CD057A3B70D2FEF` _newaddedeffectduration) (`NewAddedEffectStun_78_7F3465F4484DDAE04B87EA9D5A3B9431` _newaddedeffectstun)) (break `/Game/RPG/Blueprints/Skills/Data/S_PassiveSkillSettings` (`local.Support`)))
  (bind ((`NewAddedEffectInterval_72_ED90BC2940A78CFC4E9D5E90B9DD95C1` _newaddedeffectinterval_2) (`NewAddedEffectDuration_73_3872F84042C7C0283CD057A3B70D2FEF` _newaddedeffectduration_2) (`NewAddedEffectKnock_79_5FCF30684208CA7FCC422F920A570E91` _newaddedeffectknock)) (break `/Game/RPG/Blueprints/Skills/Data/S_PassiveSkillSettings` (`local.Support`)))
  (bind ((`NewAddedEffectDamage_75_87730A614C5DA29B44D8F69B2568AB95` _newaddedeffectdamage) (`NewAddedEffectDamageType_76_0E3E4F5B44397CEA50B6D0BC11328ED9` _newaddedeffectdamagetype) (`NewAddedEffectInterval_72_ED90BC2940A78CFC4E9D5E90B9DD95C1` _newaddedeffectinterval_3) (`NewAddedEffectDuration_73_3872F84042C7C0283CD057A3B70D2FEF` _newaddedeffectduration_3)) (break `/Game/RPG/Blueprints/Skills/Data/S_PassiveSkillSettings` (`local.Support`)))
  (bind ((`NewAddedEffect_MovSlow_Percent_77_A53FA7F542C368BF920031B6691611BD` _newaddedeffect_movslow_percent) (`NewAddedEffectInterval_72_ED90BC2940A78CFC4E9D5E90B9DD95C1` _newaddedeffectinterval_4) (`NewAddedEffectDuration_73_3872F84042C7C0283CD057A3B70D2FEF` _newaddedeffectduration_4)) (break `/Game/RPG/Blueprints/Skills/Data/S_PassiveSkillSettings` (`local.Support`)))
  (`|ExecutionSequence`
    (:`then_0`
      (`|ExecutionSequence`
        (:`then_0`
          (for _array_element (`local.Passives`)
            (if (<= (`KismetMathLibrary.RandomFloatInRange` 0.0 100.0) (`.SupportTriggerChance_31_C5F9BD5347E00E2A1705579F3D33AD2A` (break `/Game/RPG/Blueprints/Skills/Data/S_PassiveSkillSettings` _array_element)))
              (set `local.Support` _array_element)
              (`|ExecutionSequence`
                (:`then_0`
                  (if (> _newaddedeffectdamage 0.0)
                    (`KismetArrayLibrary.Array_Add` (`local.NewEffects`) (make `/Game/RPG/Blueprints/Skills/Data/S_SkillEffects` (`KismetStringLibrary.Conv_StringToName` (`KismetStringLibrary.Concat_StrStr` "Support_AddedDamage_" (`KismetStringLibrary.Conv_NameToString` (`local.SupportedSkill`)))) "NewEnumerator1" 100.0 false (`KismetMathLibrary.SelectFloat` _newaddedeffectinterval_3 1.0 (< _newaddedeffectinterval_3 0.0)) _newaddedeffectduration_3 _newaddedeffectdamage _newaddedeffectdamagetype))))
                (:`then_1`
                  (if (> _newaddedeffect_movslow_percent 0.0)
                    (`KismetArrayLibrary.Array_Add` (`local.NewEffects`) (make `/Game/RPG/Blueprints/Skills/Data/S_SkillEffects` (`KismetStringLibrary.Conv_StringToName` (`KismetStringLibrary.Concat_StrStr` "Support_MovSlow_" (`KismetStringLibrary.Conv_NameToString` (`local.SupportedSkill`)))) "NewEnumerator1" 100.0 true _newaddedeffectinterval_4 _newaddedeffectduration_4 0.0 "/Game/RPG/Blueprints/Skills/DamageTypes/BP_PhysicalDamage.BP_PhysicalDamage_C" 0.0 0.0 0.0 0.0 _newaddedeffect_movslow_percent))))
                (:`then_2`
                  (if _newaddedeffectstun
                    (`KismetArrayLibrary.Array_Add` (`local.NewEffects`) (make `/Game/RPG/Blueprints/Skills/Data/S_SkillEffects` :`SkillUniqueID` (`KismetStringLibrary.Conv_StringToName` (`KismetStringLibrary.Concat_StrStr` "Support_Stun_" (`KismetStringLibrary.Conv_NameToString` (`local.SupportedSkill`)))) :`ApplyOnce` true :`IntervalInSeconds` _newaddedeffectinterval :`DurationInSeconds` _newaddedeffectduration :`DamageType` "/Game/RPG/Blueprints/Skills/DamageTypes/BP_PhysicalDamage.BP_PhysicalDamage_C" :`ApplyStun` true))))
                (:`then_3`
                  (if _newaddedeffectknock
                    (`KismetArrayLibrary.Array_Add` (`local.NewEffects`) (make `/Game/RPG/Blueprints/Skills/Data/S_SkillEffects` :`SkillUniqueID` (`KismetStringLibrary.Conv_StringToName` (`KismetStringLibrary.Concat_StrStr` "Support_Knock_" (`KismetStringLibrary.Conv_NameToString` (`local.SupportedSkill`)))) :`ApplyOnce` true :`IntervalInSeconds` _newaddedeffectinterval_2 :`DurationInSeconds` _newaddedeffectduration_2 :`DamageType` "/Game/RPG/Blueprints/Skills/DamageTypes/BP_PhysicalDamage.BP_PhysicalDamage_C" :`ApplyKnock?` true))))))))
        (:`then_1`
          (`KismetArrayLibrary.Array_Append` Effects (`local.NewEffects`))
          (for _array_element_2 Passives
            (bind ((`SupportTriggerChance_31_C5F9BD5347E00E2A1705579F3D33AD2A` _supporttriggerchance) (`SupportEffectsDamageIncrease_Percent_67_EB8FBB18492E86406236C2A6CCCB166B` _supporteffectsdamageincrease_percent) (`SupportEffectsAddedMovement_Percent_88_48646B9F40E4FEB9D64E5F8CA694840C` _supporteffectsaddedmovement_percent) (`SupportEffectsDurationIncrease_42_FEE9DF464685AFD4FEE262A4044C60F3` _supporteffectsdurationincrease)) (break `/Game/RPG/Blueprints/Skills/Data/S_PassiveSkillSettings` _array_element_2))
            (if (<= (`KismetMathLibrary.RandomFloatInRange` 0.0 100.0) _supporttriggerchance)
              (for _index (range (`KismetArrayLibrary.Array_Length` (`local.Effects`)))
                (bind _output (`|GetArrayItem` (`local.Effects`) _index))
                (bind ((`DurationInSeconds_25_4E3939C745BEC221F153B396AF15B6D4` _durationinseconds) (`Damage_18_9FF49EE540C433C98E392EB6C7988183` _damage) (`MovementSpeedBoostSlow_Percent_50_4AB87C6249C89DA61E06AB97F23294D1` _movementspeedboostslow_percent)) (break `/Game/RPG/Blueprints/Skills/Data/S_SkillEffects` _output))
                (setmembers `/Game/RPG/Blueprints/Skills/Data/S_SkillEffects` :`StructRef` _output :`DurationInSeconds` (+ _durationinseconds _supporteffectsdurationincrease) :`Damage` (* _damage (+ (/ _supporteffectsdamageincrease_percent 100.0) 1.0)) :`MovementSpeedBoost/Slow_Percent` (`KismetMathLibrary.SelectFloat` (+ _movementspeedboostslow_percent _supporteffectsaddedmovement_percent) 0.0 (!= _movementspeedboostslow_percent 0.0)))))))))
    (:`then_1`
      (return Effects))))

(fn `GetActionbartByClass`
  (params (Class :type "/Game/RPG/Blueprints/InventorySystem/JigSaw/Data/E_ClassTypes Enum" :default "NewEnumerator0"))
  (returns (InitialActionBar :type "/Game/RPG/Blueprints/Skills/Data/S_PlayerActionbarSkills Structure"))
  (for _array_element (`self.SkillTreeConfigByClass`)
    (bind ((`Class_5_B115D9364370132981C629894C69B7BF` _class) (`InitialActionBar_13_301F4BC8427F1AF36DD190A30A41DA39` _initialactionbar)) (break `/Game/RPG/Blueprints/Skills/Data/S_SkillTreesConfig` _array_element))
    (if (`|EnumEquality` _class Class)
      (return _initialactionbar)))
  (return))

(fn `GetActiveSkillUIDs`
  (returns (SkillUIDs :type "Array of Name"))
  (locals (UIDs :type "Array of Name"))
  (for _array_element (`self.SkillTreeConfigByClass`)
    (bind (_treewidget _class _initialactionbar _servertree) (break `/Game/RPG/Blueprints/Skills/Data/S_SkillTreesConfig` _array_element))
    (if (`|EnumEquality` _class (`self.PlayerClass`))
      (for _array_element_2 _servertree
        (bind ((`RequiredLevel_25_7DD4431740BE18B8B1D721A3CEF7051D` _requiredlevel) (`UniqueID_2_C0E7A2EE4812001E2B57799EB905E4A6` _uniqueid) (`Enabled_11_562753834EB4B0783A2088B1158BE883` _enabled)) (break `/Game/RPG/Blueprints/Skills/Data/S_SkillTreeServerConfig` _array_element_2))
        (if _enabled
          (`KismetArrayLibrary.Array_Add` (`local.UIDs`) _uniqueid)))))
  (return (`local.UIDs`)))

(fn `GetSaveData`
  (returns (PlayerActiveSkills :type "Array of Name") (CurrentSkillPoints :type Integer))
  (locals (ActiveSkills :type "Array of Name (by ref)"))
  (`|ExecutionSequence`
    (:`then_0`
      (for _array_element (`self.SkillTreeConfigByClass`)
        (bind (_treewidget _class _initialactionbar _servertree) (break `/Game/RPG/Blueprints/Skills/Data/S_SkillTreesConfig` _array_element))
        (if (`|EnumEquality` _class (`self.PlayerClass`))
          (`|ExecutionSequence`
            (:`then_0`
              (for _array_element_2 _servertree
                (bind ((`RequiredLevel_25_7DD4431740BE18B8B1D721A3CEF7051D` _requiredlevel) (`UniqueID_2_C0E7A2EE4812001E2B57799EB905E4A6` _uniqueid) (`Enabled_11_562753834EB4B0783A2088B1158BE883` _enabled)) (break `/Game/RPG/Blueprints/Skills/Data/S_SkillTreeServerConfig` _array_element_2))
                (if _enabled
                  (`KismetArrayLibrary.Array_Add` (`local.ActiveSkills`) _uniqueid))))
            (:`then_1`
              (return (`local.ActiveSkills`) (`self.CurrentSkillPoints`)))))))
    (:`then_1`
      (return (`|MakeArray`) (`self.CurrentSkillPoints`)))))

(fn `GetServerTree`
  (returns (ServerTree :type "Array of /Game/RPG/Blueprints/Skills/Data/S_SkillTreeServerConfig Structure") (`Array Index` :type Integer))
  (for (_array_element _array_index) (`self.SkillTreeConfigByClass`)
    (bind ((`Class_5_B115D9364370132981C629894C69B7BF` _class) (`InitialActionBar_13_301F4BC8427F1AF36DD190A30A41DA39` _initialactionbar) (`ServerTree_9_E192F2D5432F3ABDE7AF729D2020D127` _servertree)) (break `/Game/RPG/Blueprints/Skills/Data/S_SkillTreesConfig` _array_element))
    (if (`|EnumEquality` _class (`self.PlayerClass`))
      (return _servertree _array_index)))
  (return (`|MakeArray`) 0))

(fn `GetSkillSupportPassives`
  (params (ActiveSkillID :type Name))
  (returns (SkillSupports :type "Array of /Game/RPG/Blueprints/Skills/Data/S_PassiveSkillSettings Structure"))
  (locals (Supports :type "Array of /Game/RPG/Blueprints/Skills/Data/S_PassiveSkillSettings Structure"))
  (bind _servertree (`self.GetServerTree`))
  (for _array_element _servertree
    (bind ((`RequiredLevel_25_7DD4431740BE18B8B1D721A3CEF7051D` _requiredlevel) (`SkillTree_ID_17_F547D1C14241E0AF5C480BB30C681D5D` _skilltree_id) (`SupportingSkill_ID_19_277A7E2D42F0C4534671148B9FCC5480` _supportingskill_id) (`Enabled_11_562753834EB4B0783A2088B1158BE883` _enabled) (`PassiveSettings_22_284D21D5482104C54DDB75B62C277801` _passivesettings)) (break `/Game/RPG/Blueprints/Skills/Data/S_SkillTreeServerConfig` _array_element))
    (if (and (== _supportingskill_id (`local.ActiveSkillID`)) _enabled)
      (`KismetArrayLibrary.Array_Add` (`local.Supports`) _passivesettings)))
  (return (`local.Supports`)))

(fn `GetTreeWidget`
  (returns (TreeWidgetRef :type "UserWidget Object Reference"))
  (return (`self.TreeWidgetRef`)))

(fn `GetTreeWidgetByClass`
  (params (Class :type "/Game/RPG/Blueprints/InventorySystem/JigSaw/Data/E_ClassTypes Enum" :default "NewEnumerator0"))
  (returns (TreeWidget :type "UserWidget Class Reference"))
  (for _array_element (`self.SkillTreeConfigByClass`)
    (bind ((`TreeWidget_10_DFF0056B48114A243DDE2D83FDF6CCF9` _treewidget) (`Class_5_B115D9364370132981C629894C69B7BF` _class)) (break `/Game/RPG/Blueprints/Skills/Data/S_SkillTreesConfig` _array_element))
    (if (`|EnumEquality` _class Class)
      (return _treewidget)))
  (return null))

(fn `HandleAllocatingSkillPoints`
  (params (SkillUniqueIDs :type "Array of Name (by ref)"))
  (locals (UID :type Name))
  (if (<= (`KismetArrayLibrary.Array_Length` SkillUniqueIDs) (`self.CurrentSkillPoints`))
    (for (_array_element _array_index) (`self.SkillTreeConfigByClass`)
      (bind ((`Class_5_B115D9364370132981C629894C69B7BF` _class) (`ServerTree_9_E192F2D5432F3ABDE7AF729D2020D127` _servertree)) (break `/Game/RPG/Blueprints/Skills/Data/S_SkillTreesConfig` _array_element))
      (if (`|EnumEquality` _class (`self.PlayerClass`))
        (`|ExecutionSequence`
          (:`then_0`
            (for (_array_element_2 _array_index_2) _servertree
              (bind ((`RequiredLevel_25_7DD4431740BE18B8B1D721A3CEF7051D` _requiredlevel) (`SkillTree_ID_17_F547D1C14241E0AF5C480BB30C681D5D` _skilltree_id) (`UniqueID_2_C0E7A2EE4812001E2B57799EB905E4A6` _uniqueid) (`IsPassive?_13_235D4F4C45C888DF0C8576AA0E426F60` _ispassive_) (`Enabled_11_562753834EB4B0783A2088B1158BE883` _enabled) (`PassiveSettings_22_284D21D5482104C54DDB75B62C277801` _passivesettings)) (break `/Game/RPG/Blueprints/Skills/Data/S_SkillTreeServerConfig` _array_element_2))
              (bind _output_get (set `local.UID` _uniqueid))
              (if (and (`KismetArrayLibrary.Array_Contains` (`local.SkillUniqueIDs`) _output_get) (not _enabled))
                (setmembers `/Game/RPG/Blueprints/Skills/Data/S_SkillTreeServerConfig` :`StructRef` (`|GetArrayItem` (`.ServerTree_9_E192F2D5432F3ABDE7AF729D2020D127` (break `/Game/RPG/Blueprints/Skills/Data/S_SkillTreesConfig` (`|GetArrayItem` (`self.SkillTreeConfigByClass`) _array_index))) _array_index_2) :`Enabled` true)
                (`/Engine/EditorBlueprintResources/StandardMacros.DecrementInt` (`self.CurrentSkillPoints`)
                  (:`  `
                    (if _ispassive_
                      (bind ((`SupportEffectsAddedMovement_Percent_88_48646B9F40E4FEB9D64E5F8CA694840C` _supporteffectsaddedmovement_percent) (`CharacterAddedStats_83_485627514FCE18E2CFE3F6B078CB63C3` _characteraddedstats)) (break `/Game/RPG/Blueprints/Skills/Data/S_PassiveSkillSettings` _passivesettings))
                      ;[0.1562 0.1562 0.1562] If passive skill is a stat skill then add the stats to the character
                      (if (`KismetArrayLibrary.Array_IsValidIndex` _characteraddedstats)
                        (bind _actorref (message `/Game/RPG/Blueprints/Interfaces/BPI_Controller.GetControlledPawnRef` (`self.GetOwner`)))
                        (`/Engine/EditorBlueprintResources/StandardMacros.IsValid` _actorref
                          (:`Is Valid`
                            (message `/Game/RPG/Blueprints/Interfaces/BPI_CharacterInventory.JigOnItemEquipped` _actorref (make `/Game/RPG/Blueprints/InventorySystem/JigSaw/Data/S_ItemInfo` :`ItemID` (`local.UID`) :`Name` "Item name" :`Description` "Some description.." :`ItemStats` _characteraddedstats :`DragSound` null :`DropSound` null) (`|MakeArray`) true))))))))))
          (:`then_1`
            (return)))))
    (else
      (`self.CLIENT_SetActiveTreeSkills` (`self.GetActiveSkillUIDs`) (`self.CurrentSkillPoints`)))))

(fn `OnSaveLoaded`
  (params (ActiveSkills :type "Array of Name (by ref)") (Points :type Integer) (PlayerClass :type "/Game/RPG/Blueprints/InventorySystem/JigSaw/Data/E_ClassTypes Enum" :default "NewEnumerator0"))
  (bind _skilltreeconfigbyclass (`self.SkillTreeConfigByClass`))
  (set `self.PlayerClass` PlayerClass)
  (set `self.CurrentSkillPoints` Points)
  (for (_array_element _array_index) _skilltreeconfigbyclass
    (if (`|EnumEquality` (`.Class_5_B115D9364370132981C629894C69B7BF` (break `/Game/RPG/Blueprints/Skills/Data/S_SkillTreesConfig` _array_element)) (`self.PlayerClass`))
      (bind (_treewidget _class _initialactionbar _servertree) (break `/Game/RPG/Blueprints/Skills/Data/S_SkillTreesConfig` (`|GetArrayItem` _skilltreeconfigbyclass _array_index)))
      (for (_array_element_2 _array_index_2) _servertree
        (setmembers `/Game/RPG/Blueprints/Skills/Data/S_SkillTreeServerConfig` :`StructRef` (`|GetArrayItem` _servertree _array_index_2) :`Enabled` (`KismetArrayLibrary.Array_Contains` (`local.ActiveSkills`) (`.UniqueID_2_C0E7A2EE4812001E2B57799EB905E4A6` (break `/Game/RPG/Blueprints/Skills/Data/S_SkillTreeServerConfig` _array_element_2))))))))

(fn `OnSkillPointGained`
  (params (Gained :type Integer))
  (bind _output_get (set `self.CurrentSkillPoints` (+ (stale _output_get) Gained))))

(fn `ResetSkillPoints`
  (returns (StatsToRemove :type "Array of /Game/RPG/Blueprints/InventorySystem/JigSaw/Data/S_ItemStats Structure"))
  (locals (RemoveStats :type "Array of /Game/RPG/Blueprints/InventorySystem/JigSaw/Data/S_ItemStats Structure"))
  (bind _skilltreeconfigbyclass (`self.SkillTreeConfigByClass`))
  (for (_array_element _array_index) _skilltreeconfigbyclass
    (bind ((`Class_5_B115D9364370132981C629894C69B7BF` _class) (`ServerTree_9_E192F2D5432F3ABDE7AF729D2020D127` _servertree)) (break `/Game/RPG/Blueprints/Skills/Data/S_SkillTreesConfig` _array_element))
    (if (`|EnumEquality` _class (`self.PlayerClass`))
      (`|ExecutionSequence`
        (:`then_0`
          (for (_array_element_2 _array_index_2) _servertree
            (bind ((`Enabled_11_562753834EB4B0783A2088B1158BE883` _enabled) (`PassiveSettings_22_284D21D5482104C54DDB75B62C277801` _passivesettings)) (break `/Game/RPG/Blueprints/Skills/Data/S_SkillTreeServerConfig` _array_element_2))
            (if _enabled
              (`/Engine/EditorBlueprintResources/StandardMacros.IncrementInt` (`self.CurrentSkillPoints`)
                (:`  `
                  (`KismetArrayLibrary.Array_Append` (`local.RemoveStats`) (`.CharacterAddedStats_83_485627514FCE18E2CFE3F6B078CB63C3` (break `/Game/RPG/Blueprints/Skills/Data/S_PassiveSkillSettings` _passivesettings)))
                  (setmembers `/Game/RPG/Blueprints/Skills/Data/S_SkillTreeServerConfig` :`StructRef` (`|GetArrayItem` (`.ServerTree_9_E192F2D5432F3ABDE7AF729D2020D127` (break `/Game/RPG/Blueprints/Skills/Data/S_SkillTreesConfig` (`|GetArrayItem` _skilltreeconfigbyclass _array_index))) _array_index_2) :`Enabled` false))))))
        (:`then_1`
          (`self.CLIENT_OnSkillPointsReset` (`self.CurrentSkillPoints`))
          (return (`local.RemoveStats`))))))
  (return (`|MakeArray`)))