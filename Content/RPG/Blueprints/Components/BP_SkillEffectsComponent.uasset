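; Actor component that manages timed skill effects (buffs, debuffs, damage over time) on its owner.
; ApplyEffect adds effects after alive, chance and stun/slow immunity checks, either refreshing a matching skill ID or storing under a random key in paired effect and tracker maps.
; Tick advances interval and duration timers, messaging the owner to apply, expire or remove effects.
; Helpers cleanse negative effects, clear all, and restore stat buffs with inventory component icons.
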(event `ApplyEffect`
  (params (CausedBy :type "Actor Object Reference") (Effect :type "/Game/RPG/Blueprints/Skills/Data/S_SkillEffects Structure"))
  ;[1 1 1] Add new effect
  (bind _result (message `/Game/RPG/Blueprints/Interfaces/BPI_SkillEffects.Skill_IsAlive` (`self.GetOwner`)))
  (if _result
    (`self.AddNewEffect` CausedBy Effect)))

(event `self.ReceiveTick`
  (params (DeltaSeconds :type "Float (single-precision)"))
  ;[1 1 1] Tick effects
  (if (> (`BlueprintMapLibrary.Map_Length` (`self.ListOfEffects`)) 0)
    (bind _keys (`BlueprintMapLibrary.Map_Keys` (`self.ListOfEffects`)))
    (bind (_arrayindex _arrayelement) (`/Engine/EditorBlueprintResources/StandardMacros.ReverseForEachLoop` _keys)
      (:`LoopBody`
        (`self.ProcessEffect` _arrayelement DeltaSeconds)))))

(fn `AddNewEffect`
  (params (CausedBy :type "Actor Object Reference") (Effect :type "/Game/RPG/Blueprints/Skills/Data/S_SkillEffects Structure (by ref)"))
  (locals (UniqueID :type Integer :default 0) (NewID :type Name) (TempTrack :type "/Game/RPG/Blueprints/Skills/Data/S_SkillEffect_Tracker Structure") (RefreshSkill :type "/Game/RPG/Blueprints/Skills/Data/S_SkillEffects Structure") (Index :type Integer))
  (bind ((`SkillUniqueID_35_4C0D408F4400E67044D857837E66DFA6` _skilluniqueid) (`MultipleTriggerBehavior_52_BAC88B0044DA071CA11CE8BDE635CDCF` _multipletriggerbehavior) (`EffectChance_28_831ED7FE487CE9E8A5E5398A7AF5DA78` _effectchance)) (break `/Game/RPG/Blueprints/Skills/Data/S_SkillEffects` Effect))
  (set `local.NewID` _skilluniqueid)
  (if (< (`KismetMathLibrary.RandomFloatInRange` 0.0 100.0) _effectchance)
    (bind _isimmune_ (`self.CheckImmunity` Effect))
    (if _isimmune_
      (return)
      (else
        (`|ExecutionSequence`
          (:`then_0`
            (if (`|EnumEquality` _multipletriggerbehavior "NewEnumerator1")
              (if (== _skilluniqueid "None")
                (`KismetSystemLibrary.PrintString` "SkillUniqueID is None please give you skill a valid unique ID." true true (struct :`R` 1.0 :`A` 1.0) 8.0)
                (return)
                (else
                  (bind _values (`BlueprintMapLibrary.Map_Values` (`self.ListOfEffects`)))
                  (for (_array_element _array_index) _values
                    (set `local.Index` _array_index)
                    (if (== (`.SkillUniqueID_35_4C0D408F4400E67044D857837E66DFA6` (break `/Game/RPG/Blueprints/Skills/Data/S_SkillEffects` _array_element)) (`local.NewID`))
                      (set `local.RefreshSkill` _array_element)
                      (bind _keys (`BlueprintMapLibrary.Map_Keys` (`self.ListOfEffects`)))
                      (bind _output (`|GetArrayItem` _keys (`local.Index`)))
                      (bind _output_get (set `local.TempTrack` (`BlueprintMapLibrary.Map_Find` (`self.EffectTracker`) _output)))
                      (bind _structout (setmembers `/Game/RPG/Blueprints/Skills/Data/S_SkillEffect_Tracker` :`StructRef` _output_get :`DurationTracker` 0.0))
                      (`BlueprintMapLibrary.Map_Add` (`self.EffectTracker`) _output _structout)
                      (message `/Game/RPG/Blueprints/Interfaces/BPI_SkillEffects.Skill_OnEffectRefreshed` (`self.GetOwner`) (`local.RefreshSkill`) _output)
                      (return)))))))
          (:`then_1`
            (bind _output_get_2 (set `local.UniqueID` (`KismetMathLibrary.RandomIntegerInRange` 0 2147483646)))
            (`BlueprintMapLibrary.Map_Add` (`self.ListOfEffects`) _output_get_2 Effect)
            (`BlueprintMapLibrary.Map_Add` (`self.EffectTracker`) (`local.UniqueID`) (make `/Game/RPG/Blueprints/Skills/Data/S_SkillEffect_Tracker` CausedBy))
            (message `/Game/RPG/Blueprints/Interfaces/BPI_SkillEffects.Skill_OnEffectAdded` (`self.GetOwner`) (`local.Effect`) (`local.UniqueID`))))))))

(fn `AI_RemoveNegativeEffects`
  (params (AISkillInfo :type "/Game/RPG/Blueprints/AI/Data/S_AISkillInfo Structure (by ref)"))
  (locals (RemoveEffects :type "Array of Name") (EffectID :type Name))
  (bind ((`CleanseDamageOverTime_74_897E62404FB393B3EEFD1DBAB9F6EDE9` _cleansedamageovertime) (`RemovesStunEffect_81_27CD7E5C4516C30FC2DDDBAABF7034F5` _removesstuneffect) (`RemovesMovementSlowEffect_82_0B6928454C75D688D7CF58AC33489140` _removesmovementsloweffect)) (break `/Game/RPG/Blueprints/AI/Data/S_AISkillInfo` AISkillInfo))
  ;[1 1 1] Remove negative effects
  (if (or (`KismetArrayLibrary.Array_IsValidIndex` _cleansedamageovertime) _removesstuneffect _removesmovementsloweffect)
    (bind _values (`BlueprintMapLibrary.Map_Values` (`self.ListOfEffects`)))
    (for _array_element _values
      (bind ((`SkillUniqueID_35_4C0D408F4400E67044D857837E66DFA6` _skilluniqueid) (`Damage_18_9FF49EE540C433C98E392EB6C7988183` _damage) (`DamageType_19_C26B815143BD75521AD53C969BB7031E` _damagetype) (`MovementSpeedBoostSlow_Percent_50_4AB87C6249C89DA61E06AB97F23294D1` _movementspeedboostslow_percent) (`ApplyStun_23_54E0C953455374E76BBBB5AEC4B8AF8B` _applystun)) (break `/Game/RPG/Blueprints/Skills/Data/S_SkillEffects` _array_element))
      (set `local.EffectID` _skilluniqueid)
      (`|ExecutionSequence`
        (:`then_0`
          (if (and (`KismetArrayLibrary.Array_Contains` (`.CleanseDamageOverTime_74_897E62404FB393B3EEFD1DBAB9F6EDE9` (break `/Game/RPG/Blueprints/AI/Data/S_AISkillInfo` AISkillInfo)) _damagetype) (> _damage 0.0))
            (`KismetArrayLibrary.Array_Add` (`local.RemoveEffects`) (`local.EffectID`) :!label _label)))
        (:`then_1`
          (if (and _applystun _removesstuneffect)
            (goto _label)))
        (:`then_2`
          (if (and _removesmovementsloweffect (< _movementspeedboostslow_percent 0.0))
            (goto _label)))))
    (for _array_element_2 (`local.RemoveEffects`)
      (`self.RemoveEffectByID` _array_element_2))))

(fn `CheckImmunity`
  (params (Effect :type "/Game/RPG/Blueprints/Skills/Data/S_SkillEffects Structure (by ref)"))
  (returns (`IsImmune?` :type Boolean))
  (bind ((`MovementSpeedBoostSlow_Percent_50_4AB87C6249C89DA61E06AB97F23294D1` _movementspeedboostslow_percent) (`ApplyStun_23_54E0C953455374E76BBBB5AEC4B8AF8B` _applystun)) (break `/Game/RPG/Blueprints/Skills/Data/S_SkillEffects` Effect))
  (`|ExecutionSequence`
    (:`then_0`
      (if _applystun
        (if (`self.IsImmunteToStun?`)
          (return true))))
    (:`then_1`
      (if (< _movementspeedboostslow_percent 0.0)
        (if (`self.IsImmunteToSlow?`)
          (return true))))
    (:`then_2`
      (return false))))

(fn `ClearAll`
  (bind _listofeffects (`self.ListOfEffects`))
  (`|ExecutionSequence`
    (:`then_0`
      (bind _keys (`BlueprintMapLibrary.Map_Keys` _listofeffects))
      (bind _values (`BlueprintMapLibrary.Map_Values` _listofeffects))
      (for (_array_element _array_index) _values
        (bind _output (`|GetArrayItem` _keys _array_index))
        (message `/Game/RPG/Blueprints/Interfaces/BPI_SkillEffects.Skill_OnEffectsEndDuration` (`self.GetOwner`) _array_element null _output)
        (message `/Game/RPG/Blueprints/Interfaces/BPI_SkillEffects.Skill_OnEffectRemoved` (`self.GetOwner`) _array_element _output)))
    (:`then_1`
      (`BlueprintMapLibrary.Map_Clear` (`self.ListOfEffects`))
      (`BlueprintMapLibrary.Map_Clear` (`self.EffectTracker`)))))

(fn `GetEffects`
  (returns (ListOfEffects :type "Map of Integer to /Game/RPG/Blueprints/Skills/Data/S_SkillEffects Structure") (EffectTracker :type "Map of Integer to /Game/RPG/Blueprints/Skills/Data/S_SkillEffect_Tracker Structure"))
  (return (`self.ListOfEffects`) (`self.EffectTracker`)))

(fn `IsImmunteToSlow?`
  (returns (Result :type Boolean))
  (bind _values (`BlueprintMapLibrary.Map_Values` (`self.ListOfEffects`)))
  (for _array_element _values
    (if (`.ImmuneToMovementSlow_60_837812374C55315FF29C608E549203BE` (break `/Game/RPG/Blueprints/Skills/Data/S_SkillEffects` _array_element))
      (return true)))
  (return false))

(fn `IsImmunteToStun?`
  (returns (Result :type Boolean))
  (bind _values (`BlueprintMapLibrary.Map_Values` (`self.ListOfEffects`)))
  (for _array_element _values
    (if (`.ImmuneToStun?_59_DE5F5D384EEED4E62035858C18B1A5C3` (break `/Game/RPG/Blueprints/Skills/Data/S_SkillEffects` _array_element))
      (return true)))
  (return false))

(fn `ProcessEffect`
  (params (UniqueID :type Integer) (Tick :type "Float (double-precision)"))
  (locals (Track :type "/Game/RPG/Blueprints/Skills/Data/S_SkillEffect_Tracker Structure") (Effect :type "/Game/RPG/Blueprints/Skills/Data/S_SkillEffects Structure"))
  (bind _uniqueid (`local.UniqueID`))
  (bind _tick (`local.Tick`))
  (bind _track (`local.Track`))
  (bind ((`MultipleTriggerBehavior_52_BAC88B0044DA071CA11CE8BDE635CDCF` _multipletriggerbehavior) (`ApplyOnce_30_6292483E4110CA2F7F16F6952D4171AE` _applyonce) (`IntervalInSeconds_16_58A0E64844E15B05AB7F41B8F0D26AE0` _intervalinseconds) (`DurationInSeconds_25_4E3939C745BEC221F153B396AF15B6D4` _durationinseconds)) (break `/Game/RPG/Blueprints/Skills/Data/S_SkillEffects` (`local.Effect`)))
  (bind ((`DurationTracker_7_7CA21FD74736E240E14C788DEAEDD322` _durationtracker) (`IntervalTracker_9_9A46F6D643185D90160B4FB7F2D034DE` _intervaltracker)) (break `/Game/RPG/Blueprints/Skills/Data/S_SkillEffect_Tracker` _track))
  (bind ((`DurationTracker_7_7CA21FD74736E240E14C788DEAEDD322` _durationtracker_2) (`IntervalTracker_9_9A46F6D643185D90160B4FB7F2D034DE` _intervaltracker_2) (`AppliedOnce_11_F13E61D64084768BBAE3E7A4CA5E91F7` _appliedonce)) (break `/Game/RPG/Blueprints/Skills/Data/S_SkillEffect_Tracker` (`local.Track`)))
  (bind ((`Causer_4_6E1B6EA24D6FA8DBA4EB4691412219C4` _causer) (`IntervalTracker_9_9A46F6D643185D90160B4FB7F2D034DE` _intervaltracker_3)) (break `/Game/RPG/Blueprints/Skills/Data/S_SkillEffect_Tracker` (`local.Track`)))
  (bind ((`DurationInSeconds_25_4E3939C745BEC221F153B396AF15B6D4` _durationinseconds_2)) (break `/Game/RPG/Blueprints/Skills/Data/S_SkillEffects` (`local.Effect`)))
  (set `local.Track` (`BlueprintMapLibrary.Map_Find` (`self.EffectTracker`) UniqueID))
  (set `local.Effect` (`BlueprintMapLibrary.Map_Find` (`self.ListOfEffects`) (`local.UniqueID`)))
  (setmembers `/Game/RPG/Blueprints/Skills/Data/S_SkillEffect_Tracker` :`StructRef` _track :`DurationTracker` (`KismetMathLibrary.SelectFloat` 0.0 (+ _durationtracker _tick) (< _durationinseconds 0.0)) :`IntervalTracker` (+ _tick _intervaltracker))
  (`|ExecutionSequence`
    (:`then_0`
      (if (or (not _applyonce) (not _appliedonce))
        (if (>= _intervaltracker_2 _intervalinseconds)
          (`|ExecutionSequence`
            (:`then_0`
              (message `/Game/RPG/Blueprints/Interfaces/BPI_SkillEffects.Skill_OnEffectsStarted` (`self.GetOwner`) (`local.Effect`) _causer (`.AppliedOnce_11_F13E61D64084768BBAE3E7A4CA5E91F7` (break `/Game/RPG/Blueprints/Skills/Data/S_SkillEffect_Tracker` (`local.Track`))) (`local.UniqueID`))
              (setmembers `/Game/RPG/Blueprints/Skills/Data/S_SkillEffect_Tracker` :`StructRef` (`local.Track`) :`AppliedOnce` true))
            (:`then_1`
              (setmembers `/Game/RPG/Blueprints/Skills/Data/S_SkillEffect_Tracker` :`StructRef` (`local.Track`) :`IntervalTracker` (- _intervaltracker_3 (`.IntervalInSeconds_16_58A0E64844E15B05AB7F41B8F0D26AE0` (break `/Game/RPG/Blueprints/Skills/Data/S_SkillEffects` (`local.Effect`))))))))))
    (:`then_1`
      (if (and (>= (`.DurationTracker_7_7CA21FD74736E240E14C788DEAEDD322` (break `/Game/RPG/Blueprints/Skills/Data/S_SkillEffect_Tracker` (`local.Track`))) _durationinseconds_2) (not (< _durationinseconds_2 0.0)))
        (message `/Game/RPG/Blueprints/Interfaces/BPI_SkillEffects.Skill_OnEffectsEndDuration` (`self.GetOwner`) (`local.Effect`) _causer (`local.UniqueID`))
        (`BlueprintMapLibrary.Map_Remove` (`self.EffectTracker`) _uniqueid)
        (`BlueprintMapLibrary.Map_Remove` (`self.ListOfEffects`) _uniqueid)
        (message `/Game/RPG/Blueprints/Interfaces/BPI_SkillEffects.Skill_OnEffectRemoved` (`self.GetOwner`) (`local.Effect`) _uniqueid)
        (return)
        (else
          (`BlueprintMapLibrary.Map_Add` (`self.EffectTracker`) (`local.UniqueID`) (`local.Track`))
          (return))))))

(fn `RemoveEffectByID`
  (params (EffectID :type Name))
  (bind _values (`BlueprintMapLibrary.Map_Values` (`self.ListOfEffects`)))
  (for (_array_element _array_index) _values
    (if (== (`.SkillUniqueID_35_4C0D408F4400E67044D857837E66DFA6` (break `/Game/RPG/Blueprints/Skills/Data/S_SkillEffects` _array_element)) (`local.EffectID`))
      (bind _keys (`BlueprintMapLibrary.Map_Keys` (`self.ListOfEffects`)))
      (bind _output (`|GetArrayItem` _keys _array_index))
      (message `/Game/RPG/Blueprints/Interfaces/BPI_SkillEffects.Skill_OnEffectsEndDuration` (`self.GetOwner`) (`BlueprintMapLibrary.Map_Find` (`self.ListOfEffects`) _output) null _output)
      (`BlueprintMapLibrary.Map_Remove` (`self.EffectTracker`) _output)
      (`BlueprintMapLibrary.Map_Remove` (`self.ListOfEffects`) _output)
      (message `/Game/RPG/Blueprints/Interfaces/BPI_SkillEffects.Skill_OnEffectRemoved` (`self.GetOwner`) _array_element _output)
      (return))))

(fn `RemoveNegativeEffects`
  (params (SkillEffect :type "/Game/RPG/Blueprints/Skills/Data/S_SkillInfo Structure (by ref)"))
  (locals (RemoveEffects :type "Array of Name") (EffectID :type Name))
  (bind ((`ExecutionMethod_86_860D0B624AAA6E8FC5AE3C8BAC25F1C8` _executionmethod) (`CanTargetFriendly?_88_FE12D56F44ED017DA81E78B6C6ED714F` _cantargetfriendly_) (`CleanseDamageOverTime_74_2428628F46E3BD7B9AD149899802F2AB` _cleansedamageovertime) (`RemovesStunEffect_79_9D4D9B23447F433A693273B9FF812C68` _removesstuneffect) (`RemovesMovementSlowEffect_81_B6A9BCA44552B657EBF5CBB76E155711` _removesmovementsloweffect)) (break `/Game/RPG/Blueprints/Skills/Data/S_SkillInfo` SkillEffect))
  ;[1 1 1] Remove negative effects
  (if (or (`KismetArrayLibrary.Array_IsValidIndex` _cleansedamageovertime) _removesstuneffect _removesmovementsloweffect)
    (bind _values (`BlueprintMapLibrary.Map_Values` (`self.ListOfEffects`)))
    (for _array_element _values
      (bind ((`SkillUniqueID_35_4C0D408F4400E67044D857837E66DFA6` _skilluniqueid) (`Damage_18_9FF49EE540C433C98E392EB6C7988183` _damage) (`DamageType_19_C26B815143BD75521AD53C969BB7031E` _damagetype) (`MovementSpeedBoostSlow_Percent_50_4AB87C6249C89DA61E06AB97F23294D1` _movementspeedboostslow_percent) (`ApplyStun_23_54E0C953455374E76BBBB5AEC4B8AF8B` _applystun)) (break `/Game/RPG/Blueprints/Skills/Data/S_SkillEffects` _array_element))
      (set `local.EffectID` _skilluniqueid)
      (`|ExecutionSequence`
        (:`then_0`
          (if (and (`KismetArrayLibrary.Array_Contains` (`.CleanseDamageOverTime_74_2428628F46E3BD7B9AD149899802F2AB` (break `/Game/RPG/Blueprints/Skills/Data/S_SkillInfo` SkillEffect)) _damagetype) (> _damage 0.0))
            (`KismetArrayLibrary.Array_Add` (`local.RemoveEffects`) (`local.EffectID`) :!label _label)))
        (:`then_1`
          (if (and _applystun _removesstuneffect)
            (goto _label)))
        (:`then_2`
          (if (and _removesmovementsloweffect (< _movementspeedboostslow_percent 0.0))
            (goto _label)))))
    (for _array_element_2 (`local.RemoveEffects`)
      (`self.RemoveEffectByID` _array_element_2))))

(fn `SetEffects`
  (params (ListOfEffects :type "Map of Integer to /Game/RPG/Blueprints/Skills/Data/S_SkillEffects Structure") (EffectTracker :type "Map of Integer to /Game/RPG/Blueprints/Skills/Data/S_SkillEffect_Tracker Structure"))
  (locals (Types :type "Array of /Game/RPG/Blueprints/Skills/Data/Enum_EffectTypes Enum") (Durations :type "Array of Float (double-precision)") (UIDs :type "Array of Integer") (Textures :type "Array of Texture2D Object Reference"))
  (bind _types (`local.Types`))
  (bind _listofeffects (`self.ListOfEffects`))
  (`|ExecutionSequence`
    (:`then_0`
      ;[1 1 1] Filter out positive effects
      (bind _keys (`BlueprintMapLibrary.Map_Keys` EffectTracker))
      (bind _values (`BlueprintMapLibrary.Map_Values` EffectTracker))
      (bind _keys_2 (`BlueprintMapLibrary.Map_Keys` ListOfEffects))
      (bind _values_2 (`BlueprintMapLibrary.Map_Values` ListOfEffects))
      (for (_array_element _array_index) _values_2
        (bind ((`DurationInSeconds_25_4E3939C745BEC221F153B396AF15B6D4` _durationinseconds) (`AddToMaxHealth_45_9D3837044C5B5933215110982B6BC449` _addtomaxhealth) (`AddToMaxMana_46_3FDF9DA5423F4EC9AED2F9B328FE950C` _addtomaxmana) (`AddedStats_56_84F230DB4B54AFDAFC85EE9CF414E5EF` _addedstats)) (break `/Game/RPG/Blueprints/Skills/Data/S_SkillEffects` _array_element))
        (if (and (> _durationinseconds 0.0) (or (`KismetArrayLibrary.Array_IsValidIndex` _addedstats) (!= _addtomaxhealth 0.0) (!= _addtomaxmana 0.0)))
          (`BlueprintMapLibrary.Map_Add` (`self.ListOfEffects`) (`|GetArrayItem` _keys_2 _array_index) _array_element)
          (`BlueprintMapLibrary.Map_Add` (`self.EffectTracker`) (`|GetArrayItem` _keys _array_index) (`|GetArrayItem` _values _array_index)))))
    (:`then_1`
      (bind _inv (message `/Game/RPG/Blueprints/Interfaces/BPI_CharacterInventory.CharacterGetInventoryComponent` (`self.GetOwner`)))
      (bind _keys_3 (`BlueprintMapLibrary.Map_Keys` _listofeffects))
      (bind _values_3 (`BlueprintMapLibrary.Map_Values` _listofeffects))
      (for (_array_element_2 _array_index_2) _values_3
        (bind ((`DurationInSeconds_25_4E3939C745BEC221F153B396AF15B6D4` _durationinseconds_2) (`ImmuneToStun?_59_DE5F5D384EEED4E62035858C18B1A5C3` _immunetostun_) (`ImmuneToMovementSlow_60_837812374C55315FF29C608E549203BE` _immunetomovementslow) (`EffectImage_49_65D6D9434FB96875C305DD8350528B1C` _effectimage)) (break `/Game/RPG/Blueprints/Skills/Data/S_SkillEffects` _array_element_2))
        (if (`KismetSystemLibrary.IsValid` _effectimage)
          (`KismetArrayLibrary.Array_Add` (`local.Types`) "NewEnumerator5")
          (`KismetArrayLibrary.Array_Add` (`local.Durations`) _durationinseconds_2)
          (`KismetArrayLibrary.Array_Add` (`local.UIDs`) (`|GetArrayItem` _keys_3 _array_index_2))
          (`KismetArrayLibrary.Array_Add` (`local.Textures`) _effectimage)))
      (if (`KismetArrayLibrary.Array_IsValidIndex` _types)
        (`/Game/RPG/Blueprints/Components/BP_AC_General.CLIENT_AddMultipleEffects` _inv _types (`local.Durations`) (`local.UIDs`) (`local.Textures`))))))