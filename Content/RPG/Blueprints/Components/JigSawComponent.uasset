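; JigSawComponent is a grid inventory component where items occupy rectangular blocks of slots, in the style of a jigsaw inventory.
; Initialize builds a flat Slots array from the column and row counts, each slot storing an empty flag and the hosting item's ID.
; Index/column-row helpers feed GetHostingSlots, which computes an item's footprint for add, remove, move and fit checks.
; Adds can retry rotated or skip checks, and first-fit searches can ignore given slots.
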(event `Initialize`
  ;[1 1 1] Initialize Jig Inventory
  (for _index (range (* (`self.NumOfColumns`) (`self.NumOfRows`)))
    (`KismetArrayLibrary.Array_Add` (`self.Slots`) (make `/Game/RPG/Blueprints/InventorySystem/MPContainers/Data/ServerSlotInfo` _index true -1))))

(fn `AddNewItem`
  (params (UniqueID :type Integer) (ToIndex :type Integer) (Vector :type "Vector2D Structure") (`TryRotated?` :type Boolean))
  (returns (Added :type Boolean) (`AddedRotated?` :type Boolean))
  (bind (_vector_x _vector_y) (`KismetMathLibrary.BreakVector2D` (`local.Vector`)))
  (bind (_vector_x_2 _vector_y_2) (`KismetMathLibrary.BreakVector2D` (`local.Vector`)))
  ;[1 1 1] Add an item to a certain index, also check if we can add the item first
  (bind _indexarr (`self.GetHostingSlots` ToIndex Vector))
  (for _array_element _indexarr
    (if (`.Empty_1_837A097C463AA10B4D48AFB48DBCEEE1` (break `/Game/RPG/Blueprints/InventorySystem/MPContainers/Data/ServerSlotInfo` (`|GetArrayItem` (`self.Slots`) _array_element)))
      _
      (elif (and (!= _vector_x _vector_y) (`local.TryRotated?`))
        (bind _indexarr_2 (`self.GetHostingSlots` (`local.ToIndex`) (`KismetMathLibrary.MakeVector2D` _vector_y_2 _vector_x_2)))
        (for _array_element_2 _indexarr_2
          (if (not (`.Empty_1_837A097C463AA10B4D48AFB48DBCEEE1` (break `/Game/RPG/Blueprints/InventorySystem/MPContainers/Data/ServerSlotInfo` (`|GetArrayItem` (`self.Slots`) _array_element_2))))
            (return false false)))
        (for _array_element_3 _indexarr_2
          (setmembers `/Game/RPG/Blueprints/InventorySystem/MPContainers/Data/ServerSlotInfo` :`StructRef` (`|GetArrayItem` (`self.Slots`) _array_element_3) :`Empty` false :`HostingID` (`local.UniqueID`)))
        (return true true)
        (else
          (return false false)))))
  (for _array_element_4 _indexarr
    (setmembers `/Game/RPG/Blueprints/InventorySystem/MPContainers/Data/ServerSlotInfo` :`StructRef` (`|GetArrayItem` (`self.Slots`) _array_element_4) :`Empty` false :`HostingID` (`local.UniqueID`)))
  (return true false))

(fn `AttemptMoveItemToIndex`
  (params (ItemIndex :type Integer) (ItemUID :type Integer) (ToIndex :type Integer) (ItemVector :type "Vector2D Structure") (Rotated :type Boolean))
  (returns (`Moved?` :type Boolean))
  (locals (TargetSlots :type "Array of Integer"))
  (bind (_x _y) (`KismetMathLibrary.BreakVector2D` ItemVector))
  ;[1 1 1] Attempt to move an item to another index
  (`|ExecutionSequence`
    (:`then_0`
      (bind _indexarr (`self.GetHostingSlots` ToIndex (select `bool` Rotated :`false` ItemVector :`true` (`KismetMathLibrary.MakeVector2D` _y _x))))
      (bind _output_get (set `local.TargetSlots` _indexarr))
      (for _array_element _output_get
        (bind ((`Empty_1_837A097C463AA10B4D48AFB48DBCEEE1` _empty) (`HostingID_4_170955EB41F38490334C068515F5BD61` _hostingid)) (break `/Game/RPG/Blueprints/InventorySystem/MPContainers/Data/ServerSlotInfo` (`|GetArrayItem` (`self.Slots`) _array_element)))
        (if (not (or _empty (== _hostingid (`local.ItemUID`))))
          (return false)))
      (bind _indexarr_2 (`self.GetHostingSlots` ItemIndex ItemVector))
      (for _array_element_2 _indexarr_2
        (setmembers `/Game/RPG/Blueprints/InventorySystem/MPContainers/Data/ServerSlotInfo` :`StructRef` (`|GetArrayItem` (`self.Slots`) _array_element_2) :`Empty` true :`HostingID` -1))
      (for _array_element_3 (`local.TargetSlots`)
        (setmembers `/Game/RPG/Blueprints/InventorySystem/MPContainers/Data/ServerSlotInfo` :`StructRef` (`|GetArrayItem` (`self.Slots`) _array_element_3) :`Empty` false :`HostingID` (`local.ItemUID`)))
      (return true))
    (:`then_1`
      (return false))))

(fn `Blind_AddNewItem`
  (params (UniqueID :type Integer) (ToIndex :type Integer) (Vector :type "Vector2D Structure"))
  (returns (Added :type Boolean))
  ;[1 1 1] Adds the item without checking if we can add it
  (bind _indexarr (`self.GetHostingSlots` ToIndex Vector))
  (for _array_element _indexarr
    (setmembers `/Game/RPG/Blueprints/InventorySystem/MPContainers/Data/ServerSlotInfo` :`StructRef` (`|GetArrayItem` (`self.Slots`) _array_element) :`Empty` false :`HostingID` (`local.UniqueID`)))
  (return true))

(fn `CanAddToIndex`
  (params (ToIndex :type Integer) (ItemVector :type "Vector2D Structure") (IgnoreSlots :type "Array of Integer"))
  (returns (Result :type Boolean) (ToIndexes :type "Array of Integer"))
  ;[1 1 1] Checks if a certain item can be added to a certain index while also indicating certain slots that should be ignored
  (`|ExecutionSequence`
    (:`then_0`
      (if (and (< (`local.ToIndex`) (* (`self.NumOfColumns`) (`self.NumOfRows`))) (>= (`local.ToIndex`) 0))
        (bind _indexarr (`self.GetHostingSlots` (`local.ToIndex`) (`local.ItemVector`)))
        (for _array_element _indexarr
          (if (not (or (`.Empty_1_837A097C463AA10B4D48AFB48DBCEEE1` (break `/Game/RPG/Blueprints/InventorySystem/MPContainers/Data/ServerSlotInfo` (`|GetArrayItem` (`self.Slots`) _array_element))) (`KismetArrayLibrary.Array_Contains` (`local.IgnoreSlots`) _array_element)))
            (return false (`|MakeArray`))))
        (return true _indexarr)))
    (:`then_1`
      (return false (`|MakeArray`)))))

(fn `GetColumnRowBySlotIndex`
  (params (SlotIndex :type Integer))
  (returns (Column :type Integer) (Row :type Integer))
  (locals (TempColumn :type Integer) (TempRow :type Integer))
  ;[1 1 1] Get column and row using a slot index
  (set `local.TempColumn` (mod SlotIndex (`self.NumOfColumns`)))
  (set `local.TempRow` (/ (- (`local.SlotIndex`) (`local.TempColumn`)) (`self.NumOfColumns`)))
  (return (`local.TempColumn`) (`local.TempRow`)))

(fn `GetEmptySlot_IgnoreIndexes`
  (params (SlotVectorX :type "Float (double-precision)") (SlotVectorY :type "Float (double-precision)") (IgnoreIndexs :type "Array of Integer"))
  (returns (SlotIndex :type Integer) (`Found?` :type Boolean))
  (locals (SlotVX :type Integer) (SlotVY :type Integer) (CurrentIndex :type Integer) (IgnoreScan :type Boolean) (Index :type Integer))
  (bind (_column _row) (`self.GetColumnRowBySlotIndex` (`local.Index`)))
  (bind (_column_2 _row_2) (`self.GetColumnRowBySlotIndex` (`local.Index`)))
  ;[1 1 1] Find an empty slot using a vector2D and ignoring the indicated slots
  (set `local.SlotVX` (`KismetMathLibrary.FTrunc` SlotVectorX))
  (set `local.SlotVY` (`KismetMathLibrary.FTrunc` SlotVectorY))
  (`|ExecutionSequence`
    (:`then_0`
      (for _index (range (`KismetArrayLibrary.Array_Length` (`self.Slots`)))
        (bind _output_get (set `local.CurrentIndex` _index))
        (bind ((`slotIndex_6_F4FBC5A540C0051D28A25FB780BE9C85` _slotindex) (`Empty_1_837A097C463AA10B4D48AFB48DBCEEE1` _empty)) (break `/Game/RPG/Blueprints/InventorySystem/MPContainers/Data/ServerSlotInfo` (`|GetArrayItem` (`self.Slots`) _output_get)))
        (set `local.Index` _slotindex)
        (if (or _empty (`KismetArrayLibrary.Array_Contains` (`local.IgnoreIndexs`) _output_get))
          (set `local.IgnoreScan` false)
          (if (and (== (`local.SlotVX`) 1) (== (`local.SlotVY`) 1))
            (return (`local.Index`) true)
            (elif (<= (+ _column_2 (`local.SlotVX`)) (`self.NumOfColumns`))
              (if (<= (+ _row_2 (`local.SlotVY`)) (`self.NumOfRows`))
                (for _index_2 (range 1 (+ (`local.SlotVY`) 1)) :!label _label
                  (for _index_3 (range 1 (+ (`local.SlotVX`) 1))
                    (bind (_slotindex_2 _empty_2) (break `/Game/RPG/Blueprints/InventorySystem/MPContainers/Data/ServerSlotInfo` (`|GetArrayItem` (`self.Slots`) (- (`self.GetSlotIndexByColumnRow` (+ _column _index_3) (- (+ _index_2 _row) 1)) 1))))
                    (if (not (or _empty_2 (`KismetArrayLibrary.Array_Contains` (`local.IgnoreIndexs`) _slotindex_2)))
                      (set `local.IgnoreScan` true)
                      (goto _label :!via `Break`))))
                (if (not (`local.IgnoreScan`))
                  (return (`local.CurrentIndex`) true))
                (else
                  (return -1 false))))))))
    (:`then_1`
      (return -1 false))))

(fn `GetHostingSlots`
  (params (Index :type Integer) (SlotVector :type "Vector2D Structure"))
  (returns (IndexArr :type "Array of Integer"))
  (locals (HostingSlots :type "Array of Integer") (X :type Integer) (Y :type Integer) (StartingCol :type Integer) (StartingRow :type Integer))
  (bind (_x _y) (`KismetMathLibrary.BreakVector2D` SlotVector))
  (bind _startingcol (`local.StartingCol`))
  (bind (_column _row) (`self.GetColumnRowBySlotIndex` (`local.Index`)))
  ;[1 1 1] Get hosting slots using slot index and slot vector aldo taking into consideration column and row values
  (`|ExecutionSequence`
    (:`then_0`
      (set `local.X` (`KismetMathLibrary.FTrunc` _x))
      (set `local.Y` (`KismetMathLibrary.FTrunc` _y))
      (set `local.StartingCol` _column)
      (set `local.StartingRow` _row)
      (if (not (or (>= (+ (`local.StartingCol`) (`local.X`) -1) (`self.NumOfColumns`)) (> (+ 0 (`local.Y`)) (`self.NumOfRows`))))
        (for _index (range (`local.Y`))
          (for _index_2 (range _startingcol (+ (+ _startingcol (`local.X`) -1) 1))
            (`KismetArrayLibrary.Array_Add` (`local.HostingSlots`) (`self.GetSlotIndexByColumnRow` _index_2 (+ _index (`local.StartingRow`))))))))
    (:`then_1`
      (return (`local.HostingSlots`)))))

(fn `GetSlotIndexByColumnRow`
  (params (Column :type Integer) (Row :type Integer))
  (returns (ReturnValue :type Integer))
  ;[1 1 1] Get slot index using a column and row
  (return (- (* (`self.NumOfColumns`) (+ Row 1)) (- (`self.NumOfColumns`) (`local.Column`)))))

(fn `RemoveItem`
  (params (UniqueID :type Integer) (ToIndex :type Integer) (Vector :type "Vector2D Structure"))
  (returns (Removed :type Boolean))
  ;[1 1 1] Removes the item using an index and a unique ID
  (bind _indexarr (`self.GetHostingSlots` ToIndex Vector))
  (for _array_element _indexarr
    (setmembers `/Game/RPG/Blueprints/InventorySystem/MPContainers/Data/ServerSlotInfo` :`StructRef` (`|GetArrayItem` (`self.Slots`) _array_element) :`Empty` true :`HostingID` -1))
  (return true))