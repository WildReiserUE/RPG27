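; Component that shows or hides its owner's name widget based on distance to the local player's pawn.
; On BeginPlay it caches the player's inventory component and pawn, retrying until the pawn is valid, then passes the owner to the display-name widget.
; Tick compares distance against the inventory's AI or ground-item range, with OutlineOn forcing visibility, and signals visibility changes.
; Dedicated servers disable its tick.
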(event `self.ReceiveBeginPlay`
  (bind _returnvalue (`GameplayStatics.GetPlayerController` 0))
  (bind _widget (`self.Widget`))
  ;[1 1 1] BEGIN PLAY
  (if (not (`KismetSystemLibrary.IsDedicatedServer`))
    (if (`Controller.IsLocalController` _returnvalue)
      (bind _inv (message `/Game/RPG/Blueprints/Character/Interfaces/BP_ARPGControllerInterface.GetInventoryComponent` _returnvalue))
      (set `self.InvComp` _inv)
      (bind _actorref (message `/Game/RPG/Blueprints/Character/Interfaces/BP_ARPGControllerInterface.GetControlledPawnRef` _returnvalue :!label _label))
      (bind _output_get (set `self.PawnRef` _actorref))
      (`/Engine/EditorBlueprintResources/StandardMacros.IsValid` _output_get
        (:`Is Valid`
          (`/Engine/EditorBlueprintResources/StandardMacros.IsValid` _widget
            (:`Is Valid`
              (bind _asbp_display_name (cast `/Game/RPG/Blueprints/InventorySystem/JigSaw/Widgets/BP_DisplayName` (`WidgetComponent.GetUserWidgetObject` _widget)))
              (set `/Game/RPG/Blueprints/InventorySystem/JigSaw/Widgets/BP_DisplayName.ActorOwner` (`self.GetOwner`) _asbp_display_name))))
        (:`Is Not Valid`
          (`KismetSystemLibrary.Delay` 0.2)
          (goto _label)))
      (else
        (`self.SetComponentTickEnabled` false :!label _label_2)))
    (else
      (goto _label_2))))

(event `self.ReceiveTick`
  (params (DeltaSeconds :type "Float (single-precision)"))
  (bind _pawnref (`self.PawnRef`))
  (bind _invcomp (`self.InvComp`))
  ;[1 1 1] Show item name based on distance from player
  (if (and (not (`KismetSystemLibrary.IsDedicatedServer`)) (`KismetSystemLibrary.IsValid` (`self.Widget`)))
    (if (and (`Controller.IsLocalController` (`GameplayStatics.GetPlayerController` 0)) (`KismetSystemLibrary.IsValid` _pawnref))
      (set `self.CurrentVis` (`SceneComponent.IsVisible` (`self.Widget`)))
      (`SceneComponent.SetHiddenInGame` (`self.Widget`) (select `bool` (`self.OutlineOn`) :`false` (not (< (`KismetMathLibrary.VSize` (- (`Actor.K2_GetActorLocation` (`self.GetOwner`)) (`Actor.K2_GetActorLocation` _pawnref))) (`KismetMathLibrary.SelectFloat` (`/Game/RPG/Blueprints/InventorySystem/Components/BP_InventoryComponent.AINameVisibiltyDistance` _invcomp) (`/Game/RPG/Blueprints/InventorySystem/Components/BP_InventoryComponent.NameVisibiltyDistance(ItemsOnGround)` _invcomp) (`self.UseAIDistance`))))) false)
      (if (!= (`SceneComponent.IsVisible` (`self.Widget`)) (`self.CurrentVis`))
        (`self.OnVisibilityChanged` (`SceneComponent.IsVisible` (`self.Widget`)))))))