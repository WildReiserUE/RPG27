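; SaveGame object that holds the RPG's saved characters as an array of server save records keyed by UniqueID.
; SaveCharacter builds a record from identity, inventory, stats, map location, class and the effects component's active effects, while SaveCharacterClientSide takes a prebuilt one.
; Both overwrite the matching entry found by DoesSaveExist or append a new one, then immediately write the whole object to the named slot.
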(fn `DoesSaveExist`
  (params (UniqueID :type Integer))
  (returns (ReturnValue :type Boolean) (Index :type Integer))
  (for (_array_element _array_index) (`self.SavedCharacters`)
    (if (== (`.UniqueID_2_C88D06A24343502209058BB3B76FFA53` (break `/Game/RPG/Blueprints/InventorySystem/SaveSystem/S_ServerSave` _array_element)) (`local.UniqueID`))
      (return true _array_index)))
  (return false 0))

(fn `GetSaveByIndex`
  (params (Index :type Integer))
  (returns (Output :type "/Game/RPG/Blueprints/InventorySystem/SaveSystem/S_ServerSave Structure (by ref)"))
  (return (`|GetArrayItem` (`self.SavedCharacters`) Index)))

(fn `SaveCharacter`
  (params (UniqueID :type Integer) (CharacterName :type String) (InventoryData :type "/Game/RPG/Blueprints/InventorySystem/SaveSystem/SaveData Structure") (PlayerStats :type "/Game/RPG/Blueprints/Skills/S_PlayerStats Structure") (MapName :type String) (PlayerLocation :type "Vector Structure") (PlayerClass :type "/Game/RPG/Blueprints/InventorySystem/JigSaw/Data/Enums/ClassTypes Enum" :default "NewEnumerator0") (StatsAllocatorTracker :type "/Game/RPG/Blueprints/Skills/S_StatsAllocationTracker Structure") (EffectsComp :type "/Game/RPG/Blueprints/Skills/Blueprint/SkillComponent/BP_SkillEffectsComponent Object Reference") (SlotName :type String))
  (bind (_listofeffects _effecttracker) (`/Game/RPG/Blueprints/Skills/Blueprint/SkillComponent/BP_SkillEffectsComponent.GetEffects` EffectsComp))
  (bind _s_serversave (make `/Game/RPG/Blueprints/InventorySystem/SaveSystem/S_ServerSave` UniqueID CharacterName InventoryData PlayerStats MapName PlayerLocation PlayerClass StatsAllocatorTracker _listofeffects _effecttracker))
  (bind (_returnvalue _index) (`self.DoesSaveExist` UniqueID))
  (if _returnvalue
    (`KismetArrayLibrary.Array_Set` (`self.SavedCharacters`) _index _s_serversave)
    (else
      (`KismetArrayLibrary.Array_Add` (`self.SavedCharacters`) _s_serversave)))
  (`GameplayStatics.SaveGameToSlot` self SlotName))

(fn `SaveCharacterClientSide`
  (params (UniqueID :type Integer) (SaveData :type "/Game/RPG/Blueprints/InventorySystem/SaveSystem/S_ServerSave Structure (by ref)") (SlotName :type String))
  (bind (_returnvalue _index) (`self.DoesSaveExist` UniqueID))
  (if _returnvalue
    (`KismetArrayLibrary.Array_Set` (`self.SavedCharacters`) _index SaveData)
    (else
      (`KismetArrayLibrary.Array_Add` (`self.SavedCharacters`) SaveData)))
  (`GameplayStatics.SaveGameToSlot` self SlotName))