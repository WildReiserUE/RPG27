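; BP_WorldContainerSave persists the server content of multiplayer world containers in the RPG inventory system through SaveGame slots.
; SaveContent writes the content to a new save object, using the default slot name when none is given, and can then save the player's inventory component.
; LoadContent reads that slot back, returning the content or an empty failed result.
; Both operations require saving to be enabled and a valid inventory save ID.
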(event `SaveContent`
  (params (ServerContent :type "Array of /Game/RPG/Blueprints/InventorySystem/MPContainers/Data/MpContentRep Structure (by ref)") (SlotName :type String) (InvCom :type "/Game/RPG/Blueprints/InventorySystem/Components/BP_InventoryComponent Object Reference"))
  (if (and (`self.SaveContent?`) (`/Game/RPG/Blueprints/InventorySystem/Components/BP_InventoryComponent.HasValidSaveID` InvCom))
    (bind _returnvalue (`GameplayStatics.CreateSaveGameObject` "/Game/RPG/Blueprints/InventorySystem/MPContainers/BP_WorldContainerSaveClass.BP_WorldContainerSaveClass_C"))
    (set `/Game/RPG/Blueprints/InventorySystem/MPContainers/BP_WorldContainerSaveClass.ServerContent` ServerContent _returnvalue)
    (bind _returnvalue_2 (`GameplayStatics.SaveGameToSlot` _returnvalue (`KismetMathLibrary.SelectString` (`self.SaveSlotName`) SlotName (`KismetStringLibrary.IsEmpty` SlotName))))
    (if (and _returnvalue_2 (`self.AlsoSavePlayer?`))
      (`/Game/RPG/Blueprints/InventorySystem/Components/BP_InventoryComponent.SaveContent` InvCom null false))))

(fn `LoadContent`
  (params (SlotName :type String) (InvComp :type "/Game/RPG/Blueprints/InventorySystem/Components/BP_InventoryComponent Object Reference"))
  (returns (ServerContent :type "Array of /Game/RPG/Blueprints/InventorySystem/MPContainers/Data/MpContentRep Structure") (Result :type Boolean))
  (if (and (`self.SaveContent?`) (`/Game/RPG/Blueprints/InventorySystem/Components/BP_InventoryComponent.HasValidSaveID` InvComp))
    (bind _returnvalue (`GameplayStatics.LoadGameFromSlot` (`KismetMathLibrary.SelectString` (`self.SaveSlotName`) SlotName (`KismetStringLibrary.IsEmpty` SlotName))))
    (bind _asbp_world_container_save_class (cast `/Game/RPG/Blueprints/InventorySystem/MPContainers/BP_WorldContainerSaveClass` _returnvalue)
      (:`then`
        (return (`/Game/RPG/Blueprints/InventorySystem/MPContainers/BP_WorldContainerSaveClass.ServerContent` _asbp_world_container_save_class) true))
      (:`CastFailed`
        _)))
  (return (`|MakeArray`) false))